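; BP_RotatingRoom is an interactable puzzle room that turns on Interact and highlights Cube1 through custom depth when focused.
; Grabbable, interactable actors entering the blue or purple trigger box select which of two slowed timelines plays.
; Each timeline lerps the root from its saved rotation toward a yaw of that rotation's pitch plus or minus 90 degrees.
; A DoOnce blocks re-triggering until the turn finishes and the start rotation is saved again.
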(event OnComponentBeginOverlap(BoxPurp)
  (params (OverlappedComponent :type Primitive%20Component%20Object%20Reference) (OtherActor :type Actor%20Object%20Reference) (OtherComp :type Primitive%20Component%20Object%20Reference) (OtherBodyIndex :type Integer) (bFromSweep :type Boolean) (SweepResult :type Hit%20Result%20Structure%20%28by%20ref%29))
  (if (and (Utilities|DoesObjectImplementInterface OtherActor "/Game/FPPuzzleGame/Blueprints/Interfaces/BPI_Grabable.BPI_Grabable_C") (Utilities|DoesObjectImplementInterface OtherActor "/Game/FPPuzzleGame/Blueprints/Interfaces/BPI_Interact.BPI_Interact_C"))
    (Variables|Default|SetPositionToInt 1)))

(event OnComponentBeginOverlap(BoxBlue)
  (params (OverlappedComponent :type Primitive%20Component%20Object%20Reference) (OtherActor :type Actor%20Object%20Reference) (OtherComp :type Primitive%20Component%20Object%20Reference) (OtherBodyIndex :type Integer) (bFromSweep :type Boolean) (SweepResult :type Hit%20Result%20Structure%20%28by%20ref%29))
  (if (and (Utilities|DoesObjectImplementInterface OtherActor "/Game/FPPuzzleGame/Blueprints/Interfaces/BPI_Grabable.BPI_Grabable_C") (Utilities|DoesObjectImplementInterface OtherActor "/Game/FPPuzzleGame/Blueprints/Interfaces/BPI_Interact.BPI_Interact_C"))
    (Variables|Default|SetPositionToInt 0)))

(event Custom|CheckPlayRate
  (Components|Timeline|SetPlayRate (Variables|Default|GetANIM_RotateRoom01) 0.25))

(event Custom|SetStartRotation
  (Variables|Default|SetStartRot (Transformation|GetWorldRotation (Variables|Default|GetDefaultSceneRoot))))

(event Custom|ResetDoOnce
  (Utilities|FlowControl|DoOnce false) ; enters at Reset
)

(event EventBeginPlay
  (CallFunction|SetStartRotation)
  (CallFunction|CheckPlayRate))

(event EventInteract
  (Utilities|FlowControl|DoOnce false
    (:Completed
      (switch int (Variables|Default|GetPositionToInt)
        (:Default
          (CallFunction|ResetDoOnce))
        (:0
          (bind _alpha (Timeline|ANIM_RotateRoom01 PlayFromStart)
            (:Update
              (Transformation|SetRelativeRotation (Variables|Default|GetDefaultSceneRoot) (Math|Rotator|Lerp(Rotator) (Variables|Default|GetStartRot) (Math|Rotator|MakeRotator 0.0 0.0 (+ (.pitch (Variables|Default|GetStartRot)) 9e+01)) _alpha) false false))
            (:Finished
              (CallFunction|SetStartRotation)
              (CallFunction|ResetDoOnce))))
        (:1
          (bind _alpha_2 (Timeline|ANIM_RotateRoom02 PlayFromStart)
            (:Update
              (Transformation|SetRelativeRotation (Variables|Default|GetDefaultSceneRoot) (Math|Rotator|Lerp(Rotator) (Variables|Default|GetStartRot) (Math|Rotator|MakeRotator 0.0 0.0 (- (.pitch (Variables|Default|GetStartRot)) 9e+01)) _alpha_2) false false))
            (:Finished
              (CallFunction|SetStartRotation)
              (CallFunction|ResetDoOnce))))))))

(event EventSetFocus
  (params (IsFocused :type Boolean))
  (|CallParentFunction IsFocused)
  (Rendering|SetRenderCustomDepth (Variables|Default|GetCube1) IsFocused))

(fn ConstructionScript
  (|CallParentFunction))