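; Actor component that gives its owning Character a smooth crouch and uncrouch.
; BeginPlay caches capsule dimensions and crouched height, then sets the animation play rate from CrouchSpeed.
; A component timeline lerps capsule half-height between standing and crouched, calling the Character's Crouch or UnCrouch on finish.
; Uncrouching reverses the timeline only if a standing-size capsule trace on the Visibility channel is clear; that trace has debug drawing enabled.
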(event Custom|SmoothUncrouch
  (bind _characterref (Variables|DontTouch|GetCharacterRef))
  ;[0.5234 0 1] CrouchUnCrouchFunc
  (if (CallFunction|CanUnCrouch)
    (|ComponentTimeline 0.0) ; enters at Reverse
  ))

(event Custom|SmoothCrouch
  (bind _characterref (Variables|DontTouch|GetCharacterRef))
  ;[0.5234 0 1] CrouchUnCrouchFunc
  (bind (_direction _alpha) (|ComponentTimeline 0.0)
    (:Update
      (Components|Capsule|SetCapsuleHalfHeight (Variables|/Script/Engine.Character|GetCapsuleComponent (Variables|DontTouch|GetCharacterRef)) (Math|Float|Lerp (Variables|DontTouch|GetStandingHeight) (Variables|DontTouch|GetCrouchedHeight) _alpha) true))
    (:Finished
      (switch Utilities|FlowControl|Switch|SwitchonETimelineDirection _direction
        (:Forward
          (Character|Crouch _characterref))
        (:Backward
          (Character|UnCrouch _characterref))))))

(event EventBeginPlay
  (Class|ComponentTimelineLibrary|InitializeComponentTimelines)
  ;[0 0.625 1] GetCharacterInitInfos
  (bind _ascharacter (Utilities|Casting|CastToCharacter (Components|GetOwner)))
  (Variables|DontTouch|SetCharacterRef _ascharacter)
  (Variables|DontTouch|SetStandingHeight (Components|Capsule|GetScaledCapsuleHalfHeight (Variables|/Script/Engine.Character|GetCapsuleComponent _ascharacter)))
  (Variables|DontTouch|SetRadius (Variables|/Script/Engine.CapsuleComponent|GetCapsuleRadius (Variables|/Script/Engine.Character|GetCapsuleComponent _ascharacter)))
  (Variables|DontTouch|SetCrouchedHeight (Variables|/Script/Engine.CharacterMovementComponent|GetCrouchedHalfHeight (Variables|/Script/Engine.Character|GetCharacterMovement _ascharacter)))
  ;[1 0 0.4687] SetCrouchAnimationSpeed
  (Components|Timeline|SetPlayRate (Variables|Default|GetCrouchAni) (Variables|Settings|GetCrouchSpeed)))

(fn CanUnCrouch
  (bind _characterref (Variables|DontTouch|GetCharacterRef))
  (bind _standingheight (Variables|DontTouch|GetStandingHeight))
  (bind _crouchedheight (Variables|DontTouch|GetCrouchedHeight))
  (bind _returnvalue (Transformation|GetActorLocation _characterref))
  (bind _returnvalue_2 (- _standingheight _crouchedheight))
  (bind _returnvalue_3 (+ _returnvalue (Math|Vector|MakeVector 0.0 0.0 _returnvalue_2)))
  (bind _returnvalue_4 (Collision|CapsuleTraceByChannel _returnvalue_3 _returnvalue_3 (Variables|DontTouch|GetRadius) (Variables|DontTouch|GetStandingHeight) "TraceTypeQuery1" false 0 "ForDuration"))
  (return (not _returnvalue_4)))