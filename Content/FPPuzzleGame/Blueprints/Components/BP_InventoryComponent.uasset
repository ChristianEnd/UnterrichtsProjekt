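; BP_InventoryComponent is an inventory component for the first-person puzzle game, storing items as stacked item-and-amount entries.
; SearchItem matches entries by row name and branches to Found or Not Found, feeding AddItem and RemoveItem.
; AddItem increments existing stacks by one regardless of Amount, or appends a new entry with Amount.
; RemoveItem subtracts Amount and drops depleted entries, while HasItem is an empty event.
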(event Custom|RemoveItem
  (params (Item :type Data%20Table%20Row%20Handle%20Structure%20%28by%20ref%29) (Amount :type Integer))
  ;[1 1 1] DecreaseInventory
  (bind (_itemout _indexout) (Utilities|SearchItem Item)
    (:Found
      (if (> (- (.Amount (Utilities|Struct|BreakSTRUCT_InventoryItem _itemout)) Amount) 0)
        (Utilities|Array|SetArrayElem (Variables|Default|GetItems) _indexout (Utilities|Struct|MakeSTRUCT_InventoryItem (- (.Amount (Utilities|Struct|BreakSTRUCT_InventoryItem _itemout)) Amount) (.Item (Utilities|Struct|BreakSTRUCT_InventoryItem _itemout))))
        (else
          (Utilities|Array|RemoveIndex (Variables|Default|GetItems) _indexout))))))

(event Custom|HasItem
  (params (Item :type Data%20Table%20Row%20Handle%20Structure%20%28by%20ref%29)))

(event Custom|AddItem
  (params (Item :type Data%20Table%20Row%20Handle%20Structure) (Amount :type Integer))
  ;[1 1 1] AddItemToInv
  (bind (_itemout _indexout) (Utilities|SearchItem Item)
    (:Found
      (Utilities|Array|SetArrayElem (Variables|Default|GetItems) _indexout (Utilities|Struct|MakeSTRUCT_InventoryItem (+ (.Amount (Utilities|Struct|BreakSTRUCT_InventoryItem _itemout)) 1) (.Item (Utilities|Struct|BreakSTRUCT_InventoryItem _itemout)))))
    (:NotFound
      (Utilities|Array|AddUnique (Variables|Default|GetItems) (Utilities|Struct|MakeSTRUCT_InventoryItem Amount Item)))))