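; Actor component that lets its owning Character detect and interact with objects the player looks at.
; Each tick it sphere-traces forward from the owner's camera on Visibility for actors implementing BPI_Interact, with debug drawing and prints.
; It tracks the current target, toggling its focus and firing found/lost dispatchers; switching targets clears the old one before selecting the new on a later tick.
; Interact forwards an interact message to the current target.
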(event Custom|CheckForInteractables
  (bind _playercamera (Variables|Init|GetPlayerCamera)
    (:then
      ;[0 1 0.9063] CastFunctionality
      (bind _outhit (Collision|SphereTraceByChannel (Transformation|GetWorldLocation _playercamera) (+ (Transformation|GetWorldLocation _playercamera) (* (Math|Vector|GetForwardVector _playercamera) (Variables|Settings|GetTraceDistance))) (Variables|Settings|GetTraceRadius) "TraceTypeQuery1" false 0 "ForOneFrame"))
      ;[0 1 0.1328] CheckForInteractable
      (if (Utilities|DoesObjectImplementInterface (.HitActor (Collision|BreakHitResult _outhit)) "/Game/FPPuzzleGame/Blueprints/Interfaces/BPI_Interact.BPI_Interact_C")
        (bind _currentinteractable (Variables|Default|GetCurrentInteractable)
          (:then
            ;[1 0 0.9375] DeselectOldInteractable
            (if (!= _currentinteractable (.HitActor (Collision|BreakHitResult _outhit)))
              (bind _currentinteractable_2 (Variables|Default|GetCurrentInteractable :!label _label)
                (:then
                  (Class|BPIInteract|SetFocus(Message) _currentinteractable_2 false)
                  (Default|CallLostInteractable)
                  (Variables|Default|SetCurrentInteractable 0)
                  (Development|PrintString "lookAway"))
                (:else))))
          (:else
            ;[0.6641 1 0] SetNewInteractable
            (bind _output_get (Variables|Default|SetCurrentInteractable (.HitActor (Collision|BreakHitResult _outhit))))
            (Development|PrintString (Utilities|GetDisplayName _output_get))
            (Class|BPIInteract|SetFocus(Message) _output_get true)
            (Default|CallFoundInteractable)))
        (else
          (goto _label))))
    (:else)))

(event Custom|Interact
  (bind _currentinteractable (Variables|Default|GetCurrentInteractable)
    (:then
      (Class|BPIInteract|Interact(Message) _currentinteractable))
    (:else)))

(event EventBeginPlay
  ;[0 1 0.8359] GetPlayerRefs
  (bind _ascharacter (Utilities|Casting|CastToCharacter (Components|GetOwner)))
  (bind _output_get (Variables|Init|SetCharacter _ascharacter))
  (Variables|Init|SetPlayerCamera (Actor|GetComponentbyClass _output_get "/Script/Engine.CameraComponent")))

(event EventTick
  (params (DeltaSeconds :type Float%20%28single-precision%29))
  (CallFunction|CheckforInteractables))