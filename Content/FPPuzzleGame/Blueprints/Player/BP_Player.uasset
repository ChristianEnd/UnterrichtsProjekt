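; First-person puzzle game player character that handles Enhanced Input movement, look with sensitivity and Y inversion, crouch, jump and interaction.
; Crouch toggles on the ground through BPSmoothCrouchComponent, and interaction is delegated to BPInteractComp.
; Jump acts only when crouched: a sped-up timeline lerps capsule half-height back to the cached default, then jumps.
; A CanUnCrouch capsule trace checks headroom but is not called in this graph.
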(event Custom|SetupInput
  ;[0.1232 0.3213 1] Setup Input
  (Input|AddMappingContext (PlayerController|LocalPlayerSubsystems|GetEnhancedInputLocalPlayerSubsystem (Game|GetPlayerController 0)) "/Game/FPPuzzleGame/Input/IMC_Player.IMC_Player" 0 "(bIgnoreAllPressedKeysUntilRelease=True,bForceImmediately=False)"))

(event Custom|Inits
  (CallFunction|SetupInput)
  (CallFunction|GetPlayerVariabels)
  (Components|Timeline|SetPlayRate (Variables|Default|GetJumpTimeline) 5.0))

(event Custom|GetPlayerVariabels
  ;[0 0.9766 1] GetPlayerStartHeight
  (Variables|DontTouch!!!!|SetDeafualtCapsuleHeight (Variables|/Script/Engine.CapsuleComponent|GetCapsuleHalfHeight (Variables|Collision|GetCapsuleComponent)))
  (Variables|DontTouch!!!!|SetCharacterDefaultSpeed (Class|MovementComponent|GetMaxSpeed (Variables|Character|GetCharacterMovement))))

(event Input|EnhancedActionEvents|EnhancedInputActionIA_Crouch
  (params (ActionValue :type Boolean) (ElapsedSeconds :type Float%20%28double-precision%29) (TriggeredSeconds :type Float%20%28double-precision%29) (InputAction :type Input%20Action%20Object%20Reference :default "/Game/FPPuzzleGame/Input/IA_Crouch.IA_Crouch"))
  (bind _bp_smoothcrouchcomponent (Variables|Default|GetBP_SmoothCrouchComponent))
  ;[0.9922 1 0] Crouch
  (:Started
    (if (AI|Components|NavMovement|IsMovingonGround (Variables|Character|GetCharacterMovement))
      (if (Variables|Default|GetbIsCrouched)
        (Default|SmoothUncrouch _bp_smoothcrouchcomponent)
        (else
          (Default|SmoothCrouch _bp_smoothcrouchcomponent))))))

(event Input|EnhancedActionEvents|EnhancedInputActionIA_MoveFWB_BWD
  (params (ActionValue :type Float%20%28double-precision%29) (ElapsedSeconds :type Float%20%28double-precision%29) (TriggeredSeconds :type Float%20%28double-precision%29) (InputAction :type Input%20Action%20Object%20Reference :default "/Game/FPPuzzleGame/Input/IA_MoveFWB_BWD.IA_MoveFWB_BWD"))
  ;[0.5333 0.03137 0.2824] Movement
  (:Triggered
    (Pawn|Input|AddMovementInput (Transformation|GetActorForwardVector) ActionValue false)))

(event Input|EnhancedActionEvents|EnhancedInputActionIA_MoveLeftRight
  (params (ActionValue :type Float%20%28double-precision%29) (ElapsedSeconds :type Float%20%28double-precision%29) (TriggeredSeconds :type Float%20%28double-precision%29) (InputAction :type Input%20Action%20Object%20Reference :default "/Game/FPPuzzleGame/Input/IA_MoveLeftRight.IA_MoveLeftRight"))
  ;[0.5333 0.03137 0.2824] Movement
  (:Triggered
    (Pawn|Input|AddMovementInput (Transformation|GetActorRightVector) ActionValue false)))

(event Input|EnhancedActionEvents|EnhancedInputActionIA_LookUpDown
  (params (ActionValue :type Float%20%28double-precision%29) (ElapsedSeconds :type Float%20%28double-precision%29) (TriggeredSeconds :type Float%20%28double-precision%29) (InputAction :type Input%20Action%20Object%20Reference :default "/Game/FPPuzzleGame/Input/IA_LookUpDown.IA_LookUpDown"))
  (bind _verticalsensitivity (Variables|Settings|GetVerticalSensitivity))
  ;[0.5333 0.03137 0.2824] LookInput
  (:Triggered
    (if (Variables|Settings|GetInvertY)
      (Pawn|Input|AddControllerPitchInput (* ActionValue _verticalsensitivity))
      (else
        (Pawn|Input|AddControllerPitchInput (* (* ActionValue _verticalsensitivity) -1.0))))))

(event Input|EnhancedActionEvents|EnhancedInputActionIA_Turn
  (params (ActionValue :type Float%20%28double-precision%29) (ElapsedSeconds :type Float%20%28double-precision%29) (TriggeredSeconds :type Float%20%28double-precision%29) (InputAction :type Input%20Action%20Object%20Reference :default "/Game/FPPuzzleGame/Input/IA_Turn.IA_Turn"))
  ;[0.5333 0.03137 0.2824] LookInput
  (:Triggered
    (Pawn|Input|AddControllerYawInput (* ActionValue (Variables|Settings|GetHorizontalSensitivity)))))

(event Input|EnhancedActionEvents|EnhancedInputActionIA_Jump
  (params (ActionValue :type Boolean) (ElapsedSeconds :type Float%20%28double-precision%29) (TriggeredSeconds :type Float%20%28double-precision%29) (InputAction :type Input%20Action%20Object%20Reference :default "/Game/FPPuzzleGame/Input/IA_Jump.IA_Jump"))
  (:Started
    (if (Variables|Default|GetbIsCrouched)
      (bind _alpha (Timeline|JumpTimeline PlayFromStart)
        (:Update
          (Components|Capsule|SetCapsuleHalfHeight (Variables|Collision|GetCapsuleComponent) (Math|Float|Lerp (Variables|/Script/Engine.CharacterMovementComponent|GetCrouchedHalfHeight (Variables|Character|GetCharacterMovement)) (Variables|DontTouch!!!!|GetDeafualtCapsuleHeight) _alpha) true))
        (:Finished
          (Character|Jump)))))
  (:Canceled
    (Character|StopJumping :!label _label))
  (:Completed
    (goto _label)))

(event Input|EnhancedActionEvents|EnhancedInputActionIA_Interact
  (params (ActionValue :type Boolean) (ElapsedSeconds :type Float%20%28double-precision%29) (TriggeredSeconds :type Float%20%28double-precision%29) (InputAction :type Input%20Action%20Object%20Reference :default "/Game/FPPuzzleGame/Input/IA_Interact.IA_Interact"))
  (:Triggered
    (Default|Interact (Variables|Default|GetBP_InteractComp))))

(event EventBeginPlay
  (CallFunction|Inits))

(event Collision|EventActorBeginOverlap
  (params (OtherActor :type Actor%20Object%20Reference)))

(event EventTick
  (params (DeltaSeconds :type Float%20%28single-precision%29)))

(fn ConstructionScript)

(fn CanUnCrouch
  (bind _returnvalue (Transformation|GetActorLocation))
  (bind _capsulecomponent (Variables|Collision|GetCapsuleComponent))
  (bind _deafualtcapsuleheight (Variables|DontTouch!!!!|GetDeafualtCapsuleHeight))
  (bind _capsulehalfheight (Variables|/Script/Engine.CapsuleComponent|GetCapsuleHalfHeight _capsulecomponent))
  (bind _returnvalue_2 (- _deafualtcapsuleheight _capsulehalfheight))
  (bind _returnvalue_3 (+ _returnvalue (Math|Vector|MakeVector 0.0 0.0 _returnvalue_2)))
  (bind _returnvalue_4 (Collision|CapsuleTraceByChannel _returnvalue_3 _returnvalue_3 (Variables|/Script/Engine.CapsuleComponent|GetCapsuleRadius _capsulecomponent) _capsulehalfheight "TraceTypeQuery1" false 0 "ForDuration"))
  (return (not _returnvalue_4)))