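; BP_Mover is an interactable puzzle-game actor that moves a set of other actors to target locations when used.
; Interact plays a timeline at PlayRate, lerping each of ActorsToMove toward its matching Locations entry from its current position, so easing compounds each update.
; It also plays an optional Level Sequence in parallel.
; AfterAnimation fires when the timeline finishes but is empty here, as are SetFocus and CheckForItem.
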(event Custom|CheckForItem)

(event Custom|AfterAnimation)

(event EventInteract
  (bind _actorstomove (Variables|Default|GetActorsToMove))
  (bind _levelsequence (Variables|Default|GetLevelSequence))
  (Utilities|FlowControl|Sequence
    (:then_0
      ;[1 1 1] ActorToMove
      (bind _alpha (Timeline|Anim PlayFromStart)
        (:Update
          (for (_array_element _array_index) _actorstomove
            (if (Utilities|Array|IsValidIndex _actorstomove _array_index)
              (Transformation|SetActorLocation _array_element (Math|Vector|Lerp(Vector) (Transformation|GetActorLocation _array_element) (Utilities|Array|Get(acopy) (Variables|Default|GetLocations) _array_index) _alpha) false false))))
        (:Finished
          (CallFunction|AfterAnimation))))
    (:then_1
      ;[1 1 1] PlayLevelSequence
      (Utilities|IsValid _levelsequence
        (:Is%20Valid
          (Sequencer|Player|Play (Variables|/Script/LevelSequence.LevelSequenceActor|GetSequencePlayer _levelsequence) :!class /Script/MovieScene.MovieSceneSequencePlayer))))))

(event EventSetFocus
  (params (IsFocused :type Boolean)))

(event EventBeginPlay
  ;[1 1 1] SetPlayRate
  (Components|Timeline|SetPlayRate (Variables|Default|GetAnim) (Variables|Default|GetPlayRate)))

(fn ConstructionScript)