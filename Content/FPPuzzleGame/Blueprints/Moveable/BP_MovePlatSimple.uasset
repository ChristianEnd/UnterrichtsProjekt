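; BP_MovePlatSimple is a simple moving platform for a puzzle game that slides its base from its local origin to a TargetVector offset.
; A timeline drives a lerp of the relative location, with its play rate scaled inversely to travel distance so speed stays consistent.
; Start, Stop and Reverse events control the timeline, while MovePlatform only stores an AllowMove flag that these graphs do not read.
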(event Custom|MovePlatform
  (params (ShouldMove :type Boolean))
  (Variables|Default|SetAllowMove ShouldMove))

(event Custom|Reverse
  (bind _alpha (Timeline|MovementAni Reverse)
    (:Update
      (Transformation|SetRelativeLocation (Variables|Default|GetPlatformBase) (Math|Vector|Lerp(Vector) "0, 0, 0" (Variables|Default|GetTargetVector) _alpha) false false))))

(event Custom|Start
  (bind _alpha (Timeline|MovementAni Play)
    (:Update
      (Transformation|SetRelativeLocation (Variables|Default|GetPlatformBase) (Math|Vector|Lerp(Vector) "0, 0, 0" (Variables|Default|GetTargetVector) _alpha) false false))))

(event Custom|Stop
  (bind _alpha (Timeline|MovementAni Stop)
    (:Update
      (Transformation|SetRelativeLocation (Variables|Default|GetPlatformBase) (Math|Vector|Lerp(Vector) "0, 0, 0" (Variables|Default|GetTargetVector) _alpha) false false))))

(event EventTick
  (params (DeltaSeconds :type Float%20%28single-precision%29)))

(event EventBeginPlay
  (Components|Timeline|SetPlayRate (Variables|Default|GetMovementAni) (/ (Math|Float|MakeLiteralFloat 1.0) (/ (Math|Vector|VectorLength (Variables|Default|GetTargetVector)) 1e+02))))

(fn ConstructionScript)