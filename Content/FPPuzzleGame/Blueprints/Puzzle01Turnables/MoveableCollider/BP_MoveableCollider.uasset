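; Movable selection box for a turnables puzzle that picks a line of pieces and rotates them together.
; Move events step the box along local Z; FlipIt, when allowed, resets it to start and toggles horizontal/vertical.
; Overlaps write BPI_MiniGameTurnable actors into a wrapping nine-slot array, changing materials when it wraps and on end overlap.
; Turn rotates every stored actor in fixed steps, by yaw when horizontal, otherwise by roll.
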(event OnComponentBeginOverlap(Box)
  (params (OverlappedComponent :type Primitive%20Component%20Object%20Reference) (OtherActor :type Actor%20Object%20Reference) (OtherComp :type Primitive%20Component%20Object%20Reference) (OtherBodyIndex :type Integer) (bFromSweep :type Boolean) (SweepResult :type Hit%20Result%20Structure%20%28by%20ref%29))
  ;[0.2656 1 0] AddToArray
  (if (Utilities|DoesObjectImplementInterface OtherActor "/Game/FPPuzzleGame/Blueprints/Interfaces/BPI_MiniGameTurnable.BPI_MiniGameTurnable_C")
    (Utilities|Array|SetArrayElem (Variables|Default|GetActiveSelection) (Variables|Default|GetIndexCount) OtherActor true)
    (Variables|Default|SetIndexCount (+ (Variables|Default|GetIndexCount) 1))
    (if (== (Variables|Default|GetIndexCount) 9)
      (Variables|Default|SetIndexCount 0)
      (CallFunction|ChangeMatSelected))))

(event OnComponentEndOverlap(Box)
  (params (OverlappedComponent :type Primitive%20Component%20Object%20Reference) (OtherActor :type Actor%20Object%20Reference) (OtherComp :type Primitive%20Component%20Object%20Reference) (OtherBodyIndex :type Integer))
  ;[0.2656 1 0] AddToArray
  (if (Utilities|DoesObjectImplementInterface OtherActor "/Game/FPPuzzleGame/Blueprints/Interfaces/BPI_MiniGameTurnable.BPI_MiniGameTurnable_C")
    (CallFunction|ChangeBackMaterial)))

(event Custom|MoveDown/Lef
  (params (PositionInt :type Integer))
  ;[1 0 0.6328] MoveNegative
  (if (>= PositionInt 2)
    (Transformation|AddLocalOffset (Variables|Default|GetBox) (Math|Vector|MakeVector 0.0 0.0 -6e+02) false false)
    (elif (<= PositionInt -2)
      (Transformation|AddLocalOffset (Variables|Default|GetBox) (Math|Vector|MakeVector 0.0 0.0 6e+02) false false)
      (else
        (Transformation|AddLocalOffset (Variables|Default|GetBox) (Math|Vector|MakeVector 0.0 0.0 -3e+02) false false)))))

(event Custom|MoveUp/Right
  (params (PositionInt :type Integer))
  ;[0.4062 1 0] MovePositive
  (Variables|ControlValues|SetPosition%20Int PositionInt)
  (if (>= PositionInt 2)
    (Transformation|AddLocalOffset (Variables|Default|GetBox) (Math|Vector|MakeVector 0.0 0.0 6e+02) false false)
    (elif (<= PositionInt -2)
      (Transformation|AddLocalOffset (Variables|Default|GetBox) (Math|Vector|MakeVector 0.0 0.0 -6e+02) false false)
      (else
        (Transformation|AddLocalOffset (Variables|Default|GetBox) (Math|Vector|MakeVector 0.0 0.0 3e+02) false false)))))

(event Custom|FlipIt
  (params (IsHorizontal :type Boolean))
  ;[1 0 0.1641] FlipTheCollider
  (if (Variables|Default|GetIsAllowedToBeFlipped)
    (Transformation|SetWorldLocation (Variables|Default|GetBox) (Variables|ControlValues|GetStartLocation) false false)
    (Variables|ControlValues|SetPosition%20Int 0)
    (CallFunction|RotateSelecta)))

(event Custom|RotateSelecta
  (bind _box (Variables|Default|GetBox))
  ;[0.7578 1 0] RotateTheCollider
  (Utilities|FlowControl|FlipFlop
    (:A
      (Variables|ControlValues|SetIsHorizontal false)
      (Transformation|AddRelativeRotation _box (Math|Rotator|MakeRotator 0.0 9e+01 0.0) false false))
    (:B
      (Variables|ControlValues|SetIsHorizontal true)
      (Transformation|AddRelativeRotation _box (Math|Rotator|MakeRotator 0.0 -9e+01 0.0) false false))))

(event Custom|ComponentMaterialChange
  (for _array_element (Variables|Default|GetOther%20Comp)
    (Rendering|Material|SetMaterial _array_element 0 "/Game/FPPuzzleGame/Materials/General/M_MI_E_Green.M_MI_E_Green")
    (Rendering|Material|SetMaterial _array_element 0 "/Game/FPPuzzleGame/Materials/General/M_.M_")))

(event Custom|Turn
  (params (TurnDirection :type Float%20%28double-precision%29))
  (bind _activeselection (Variables|Default|GetActiveSelection))
  (bind _activeselection_2 (Variables|Default|GetActiveSelection))
  (if (Variables|ControlValues|GetIsHorizontal)
    (if (> TurnDirection 0.0)
      (for _array_element _activeselection_2
        (Transformation|AddRelativeRotation (Variables|/Script/Engine.Actor|GetRootComponent _array_element) (Math|Rotator|MakeRotator 0.0 0.0 3e+01) false false))
      (else
        (for _array_element_2 _activeselection_2
          (Transformation|AddRelativeRotation (Variables|/Script/Engine.Actor|GetRootComponent _array_element_2) (Math|Rotator|MakeRotator 0.0 0.0 -3e+01) false false))))
    (elif (> TurnDirection 0.0)
      (for _array_element_3 _activeselection
        (Transformation|AddRelativeRotation (Variables|/Script/Engine.Actor|GetRootComponent _array_element_3) (Math|Rotator|MakeRotator 3e+01 0.0 0.0) false false)
        (Development|PrintString "Hello"))
      (else
        (for _array_element_4 _activeselection
          (Transformation|AddRelativeRotation (Variables|/Script/Engine.Actor|GetRootComponent _array_element_4) (Math|Rotator|MakeRotator -3e+01 0.0 0.0) false false))))))

(event Custom|ChangeBackMaterial
  (bind _activeselection (Variables|Default|GetActiveSelection))
  (for (_ _array_index) _activeselection
    (Rendering|Material|SetMaterial (Actor|GetComponentbyClass (Utilities|Array|Get(acopy) _activeselection _array_index) "/Script/Engine.MeshComponent") 0 "/Game/FPPuzzleGame/Materials/General/M_MI_E_Green.M_MI_E_Green")
    (Rendering|Material|SetMaterial (Actor|GetComponentbyClass (Utilities|Array|Get(acopy) _activeselection _array_index) "/Script/Engine.MeshComponent") 0 "/Game/StarterContent/Materials/M_Brick_Clay_Old.M_Brick_Clay_Old")))

(event Custom|ChangeMatSelected
  (bind _activeselection (Variables|Default|GetActiveSelection))
  ;[0.2656 1 0] AddToArray
  (for (_ _array_index) _activeselection
    (Rendering|Material|SetMaterial (Actor|GetComponentbyClass (Utilities|Array|Get(acopy) _activeselection _array_index) "/Script/Engine.MeshComponent") 0 "/Game/FPPuzzleGame/Materials/General/M_MI_E_Green.M_MI_E_Green")
    (Rendering|Material|SetMaterial (Actor|GetComponentbyClass (Utilities|Array|Get(acopy) _activeselection _array_index) "/Script/Engine.MeshComponent") 0 "/Game/FPPuzzleGame/Materials/General/M_.M_")))

(event EventBeginPlay
  (Variables|ControlValues|SetStartLocation (Transformation|GetWorldLocation (Variables|Default|GetBox))))

(fn ConstructionScript)