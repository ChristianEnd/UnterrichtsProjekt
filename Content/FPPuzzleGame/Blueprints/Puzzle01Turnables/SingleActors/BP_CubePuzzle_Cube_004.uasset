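; BP_CubePuzzle_Cube_004 is a single cube actor for the turnables puzzle that highlights under the mouse cursor.
; Cursor begin and end events set IsOverlapping, which drives custom depth rendering on Cube3x3Cube, and swap its material.
; Every Tick, regardless of hover, it line-traces WorldDynamic objects along the deprojected mouse ray and stores the impact normal, which nothing in these graphs reads.
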(event MouseInput|EventActorBeginCursorOver
  (bind _cube3x3_cube (Variables|Default|GetCube3x3_Cube))
  ;[1 0.09375 0] Highlight
  (bind _output_get (Variables|Default|SetIsOverlapping true))
  (Rendering|SetRenderCustomDepth _cube3x3_cube _output_get)
  (Rendering|Material|SetMaterial _cube3x3_cube 0 "/Game/FPPuzzleGame/Materials/Buttons/M_A.M_A"))

(event MouseInput|EventActorEndCursorOver
  (bind _cube3x3_cube (Variables|Default|GetCube3x3_Cube))
  ;[1 0.09375 0] Highlight
  (bind _output_get (Variables|Default|SetIsOverlapping false))
  (Rendering|SetRenderCustomDepth _cube3x3_cube _output_get)
  (Rendering|Material|SetMaterial _cube3x3_cube 0 "/Game/StarterContent/Materials/M_Basic_Floor.M_Basic_Floor"))

(event EventTick
  (params (DeltaSeconds :type Float%20%28single-precision%29))
  (bind _returnvalue (Game|GetPlayerController 0))
  (bind (_worldlocation _worlddirection) (Game|Player|ConvertMouseLocationToWorldSpace _returnvalue))
  ;[1 0.9609 0] HierNachhernochBoolObUndNicht
  (bind _outhit (Collision|LineTraceForObjects _worldlocation (+ (* _worlddirection 1e+04) _worldlocation) (Utilities|Array|MakeArray "ObjectTypeQuery2") false 0 "None" false))
  (Variables|Default|SetImpactNormal (Math|Vector|GetVectorArrayAverage (Utilities|Array|MakeArray (.ImpactNormal (Collision|BreakHitResult _outhit))))))

(fn ConstructionScript)