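; BP_CubePuzzle_Cube_001 is a single cube actor for a turnable puzzle that responds to the mouse cursor.
; Cursor-over events set the IsOverlapping flag and toggle custom depth rendering on the Cube3x3Cube component to highlight it.
; Every tick, it line-traces WorldDynamic objects from the deprojected mouse position and stores the hit's ImpactNormal, which nothing in this file reads.
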(event MouseInput|EventActorBeginCursorOver
  ;[1 0.09375 0] Highlight
  (bind _output_get (Variables|Default|SetIsOverlapping true))
  (Rendering|SetRenderCustomDepth (Variables|Default|GetCube3x3_Cube) _output_get))

(event MouseInput|EventActorEndCursorOver
  ;[1 0.09375 0] Highlight
  (bind _output_get (Variables|Default|SetIsOverlapping false))
  (Rendering|SetRenderCustomDepth (Variables|Default|GetCube3x3_Cube) _output_get))

(event EventTick
  (params (DeltaSeconds :type Float%20%28single-precision%29))
  (bind _returnvalue (Game|GetPlayerController 0))
  (bind (_worldlocation _worlddirection) (Game|Player|ConvertMouseLocationToWorldSpace _returnvalue))
  ;[1 0.9609 0] HierNachhernochBoolObUndNicht
  (bind _outhit (Collision|LineTraceForObjects _worldlocation (+ (* _worlddirection 1e+03) _worldlocation) (Utilities|Array|MakeArray "ObjectTypeQuery2") false 0 "None" false))
  (Variables|Default|SetImpactNormal (Math|Vector|GetVectorArrayAverage (Utilities|Array|MakeArray (.ImpactNormal (Collision|BreakHitResult _outhit))))))

(fn ConstructionScript)