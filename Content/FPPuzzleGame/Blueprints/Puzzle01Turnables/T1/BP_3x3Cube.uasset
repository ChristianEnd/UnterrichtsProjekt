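; A 3x3 turnable cube puzzle for a minigame that highlights and rotates rows or columns of child cube actors.
; HighlightRow uses custom depth to mark a slice and set the selection, which TurnSelected uses to rotate each cube in that slice's array.
; Overlap volumes are meant to fill these arrays, but only the left column's begin-overlap is wired.
; It also adds the minigame input mapping and has debug-printing init and check events.
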(event OnComponentBeginOverlap(C_V_Left)
  (params (OverlappedComponent :type Primitive%20Component%20Object%20Reference) (OtherActor :type Actor%20Object%20Reference) (OtherComp :type Primitive%20Component%20Object%20Reference) (OtherBodyIndex :type Integer) (bFromSweep :type Boolean) (SweepResult :type Hit%20Result%20Structure%20%28by%20ref%29))
  ;[0 0.0625 1] VLArrayFill
  (if (Utilities|DoesObjectImplementInterface OtherActor "/Game/FPPuzzleGame/Blueprints/Interfaces/BPI_MiniGameTurnable.BPI_MiniGameTurnable_C")
    (Utilities|Array|Add (Variables|Arrays/DontTouch|GetC_V_Left_Cubes) OtherActor)))

(event OnComponentBeginOverlap(C_H_Mid)
  (params (OverlappedComponent :type Primitive%20Component%20Object%20Reference) (OtherActor :type Actor%20Object%20Reference) (OtherComp :type Primitive%20Component%20Object%20Reference) (OtherBodyIndex :type Integer) (bFromSweep :type Boolean) (SweepResult :type Hit%20Result%20Structure%20%28by%20ref%29))
  ;[0 1 0.4609] MH_ArrayFill
)

(event OnComponentEndOverlap(C_H_Mid)
  (params (OverlappedComponent :type Primitive%20Component%20Object%20Reference) (OtherActor :type Actor%20Object%20Reference) (OtherComp :type Primitive%20Component%20Object%20Reference) (OtherBodyIndex :type Integer))
  ;[0 1 0.4609] MH_ArrayFill
)

(event OnComponentBeginOverlap(C_H_Bottom)
  (params (OverlappedComponent :type Primitive%20Component%20Object%20Reference) (OtherActor :type Actor%20Object%20Reference) (OtherComp :type Primitive%20Component%20Object%20Reference) (OtherBodyIndex :type Integer) (bFromSweep :type Boolean) (SweepResult :type Hit%20Result%20Structure%20%28by%20ref%29))
  ;[0 1 1] BH_ArrayFill
)

(event OnComponentEndOverlap(C_H_Bottom)
  (params (OverlappedComponent :type Primitive%20Component%20Object%20Reference) (OtherActor :type Actor%20Object%20Reference) (OtherComp :type Primitive%20Component%20Object%20Reference) (OtherBodyIndex :type Integer))
  ;[0 1 1] BH_ArrayFill
)

(event OnComponentEndOverlap(C_V_Left)
  (params (OverlappedComponent :type Primitive%20Component%20Object%20Reference) (OtherActor :type Actor%20Object%20Reference) (OtherComp :type Primitive%20Component%20Object%20Reference) (OtherBodyIndex :type Integer))
  ;[0 0.0625 1] VLArrayFill
)

(event OnComponentBeginOverlap(C_V_Right)
  (params (OverlappedComponent :type Primitive%20Component%20Object%20Reference) (OtherActor :type Actor%20Object%20Reference) (OtherComp :type Primitive%20Component%20Object%20Reference) (OtherBodyIndex :type Integer) (bFromSweep :type Boolean) (SweepResult :type Hit%20Result%20Structure%20%28by%20ref%29))
  ;[0 1 0.7656] VRArrayFill
)

(event OnComponentEndOverlap(C_V_Right)
  (params (OverlappedComponent :type Primitive%20Component%20Object%20Reference) (OtherActor :type Actor%20Object%20Reference) (OtherComp :type Primitive%20Component%20Object%20Reference) (OtherBodyIndex :type Integer))
  ;[0 1 0.7656] VRArrayFill
)

(event OnComponentBeginOverlap(C_V_Mid)
  (params (OverlappedComponent :type Primitive%20Component%20Object%20Reference) (OtherActor :type Actor%20Object%20Reference) (OtherComp :type Primitive%20Component%20Object%20Reference) (OtherBodyIndex :type Integer) (bFromSweep :type Boolean) (SweepResult :type Hit%20Result%20Structure%20%28by%20ref%29))
  ;[0.6875 0 1] VMArrayFill
)

(event OnComponentEndOverlap(C_V_Mid)
  (params (OverlappedComponent :type Primitive%20Component%20Object%20Reference) (OtherActor :type Actor%20Object%20Reference) (OtherComp :type Primitive%20Component%20Object%20Reference) (OtherBodyIndex :type Integer))
  ;[0.6875 0 1] VMArrayFill
)

(event OnComponentEndOverlap(C_H_Top)
  (params (OverlappedComponent :type Primitive%20Component%20Object%20Reference) (OtherActor :type Actor%20Object%20Reference) (OtherComp :type Primitive%20Component%20Object%20Reference) (OtherBodyIndex :type Integer))
  ;[0.4531 1 0] TH_ArrayFill
)

(event OnComponentBeginOverlap(C_H_Top)
  (params (OverlappedComponent :type Primitive%20Component%20Object%20Reference) (OtherActor :type Actor%20Object%20Reference) (OtherComp :type Primitive%20Component%20Object%20Reference) (OtherBodyIndex :type Integer) (bFromSweep :type Boolean) (SweepResult :type Hit%20Result%20Structure%20%28by%20ref%29))
  ;[0.4531 1 0] TH_ArrayFill
)

(event Custom|InitSingleCubes
  ;[0.2422 0 1] InitSingleCubes
  (bind _output_get (Variables|Default|SetChild%20Actors (Actor|GetAllChildActors self false)))
  (for _array_element _output_get
    (Utilities|FlowControl|Delay 0.5)
    (Transformation|AddRelativeRotation (Variables|/Script/Engine.Actor|GetRootComponent _array_element) "180.000000,0.000000,0.000000" false false)
    (Development|PrintString (Utilities|GetDisplayName _array_element))))

(event Custom|SetupInput
  (params (AsPlayerController :type Player%20Controller%20Object%20Reference))
  ;[0.875 0 1] SetupInput
  (Input|AddMappingContext (PlayerController|LocalPlayerSubsystems|GetEnhancedInputLocalPlayerSubsystem AsPlayerController) "/Game/FPPuzzleGame/Input/IMC_TurnablesMiniGame.IMC_TurnablesMiniGame" 0 "(bIgnoreAllPressedKeysUntilRelease=True,bForceImmediately=False)"))

(event Custom|HighlightRow
  (params (0/1/2/3%20 :type Integer))
  (bind _c_v_left (Variables|Default|GetC_V_Left))
  (bind _c_h_top (Variables|Default|GetC_H_Top))
  (if (Variables|Default|GetIsHorizontal)
    (switch int 0/1/2/3%20
      (:0
        ;[0 1 0.1797] HighlightNone
        (Rendering|SetRenderCustomDepth _c_v_left false)
        (Variables|Default|SetSetRowToTurn 0))
      (:1
        ;[1 0.4688 0] HighlightLeft
        (Rendering|SetRenderCustomDepth _c_v_left true)
        (Variables|Default|SetSetRowToTurn 1))
      (:2
        ;[1 0.6797 0] HighlightMid
        (Rendering|SetRenderCustomDepth (Variables|Default|GetC_V_Mid) true)
        (Variables|Default|SetSetRowToTurn 2))
      (:3
        ;[0.5 1 0] HighlightBot
        (Rendering|SetRenderCustomDepth (Variables|Default|GetC_V_Right) true)
        (Variables|Default|SetSetRowToTurn 3)))
    (else
      (switch int 0/1/2/3%20
        (:0
          ;[0 1 0.1797] HighlightNone
          (Rendering|SetRenderCustomDepth _c_h_top false))
        (:1
          ;[0.2891 1 0] HighlightTop
          (Rendering|SetRenderCustomDepth _c_h_top true)
          (Variables|Default|SetSetRowToTurn 4))
        (:2
          ;[0.6875 0 1] HighlightMid
          (Rendering|SetRenderCustomDepth (Variables|Default|GetC_H_Mid) true)
          (Variables|Default|SetSetRowToTurn 5))
        (:3
          ;[1 0.7266 0] HighlightBot
          (Rendering|SetRenderCustomDepth (Variables|Default|GetC_H_Bottom) true)
          (Variables|Default|SetSetRowToTurn 6))))))

(event Custom|TurnSelected
  (params (Modifier :type Float%20%28double-precision%29))
  (Variables|Default|SetModifier Modifier)
  (switch int (Variables|Default|GetSetRowToTurn)
    (:0
      (Development|PrintString "NoneSelected"))
    (:1
      (for _array_element (Variables|Arrays/DontTouch|GetC_V_Left_Cubes)
        (Transformation|AddRelativeRotation (Variables|/Script/Engine.Actor|GetRootComponent _array_element) (Math|Rotator|MakeRotator 0.0 0.0 (* (Variables|Default|GetToRotateAmount) (Variables|Default|GetModifier))) false false)))
    (:2
      (for _array_element_2 (Variables|Arrays/DontTouch|GetC_V_Mid_Cubes)
        (Transformation|AddRelativeRotation (Variables|/Script/Engine.Actor|GetRootComponent _array_element_2) (Math|Rotator|MakeRotator 0.0 0.0 (* (Variables|Default|GetToRotateAmount) (Variables|Default|GetModifier))) false false)))
    (:3
      (for _array_element_3 (Variables|Arrays/DontTouch|GetC_V_Right_Cubes)
        (Transformation|AddRelativeRotation (Variables|/Script/Engine.Actor|GetRootComponent _array_element_3) (Math|Rotator|MakeRotator 0.0 (* (Variables|Default|GetToRotateAmount) (Variables|Default|GetModifier)) 0.0) false false)))
    (:4
      (for _array_element_4 (Variables|Arrays/DontTouch|GetC_H_Top_Cubes)
        (Transformation|AddRelativeRotation (Variables|/Script/Engine.Actor|GetRootComponent _array_element_4) (Math|Rotator|MakeRotator 0.0 (* (Variables|Default|GetToRotateAmount) (Variables|Default|GetModifier)) 0.0) false false)))
    (:5
      (for _array_element_5 (Variables|Arrays/DontTouch|GetC_H_Mid_Cubes)
        (Transformation|AddRelativeRotation (Variables|/Script/Engine.Actor|GetRootComponent _array_element_5) (Math|Rotator|MakeRotator 0.0 (* (Variables|Default|GetToRotateAmount) (Variables|Default|GetModifier)) 0.0) false false)))
    (:6
      (for _array_element_6 (Variables|Arrays/DontTouch|GetC_H_Bottom_Cubes)
        (Transformation|AddRelativeRotation (Variables|/Script/Engine.Actor|GetRootComponent _array_element_6) (Math|Rotator|MakeRotator 0.0 (* (Variables|Default|GetToRotateAmount) (Variables|Default|GetModifier)) 0.0) false false)))))

(event Custom|CheckRow
  (for _array_element (Variables|Arrays/DontTouch|GetC_H_Bottom_Cubes)
    (Development|PrintString (Utilities|GetDisplayName _array_element))))

(fn ConstructionScript)