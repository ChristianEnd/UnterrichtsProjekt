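; BP_3x3Cube is the 3x3 cube actor for the turnables puzzle, with custom-depth highlighting of one row or column.
; Six overlap volumes store "Cube"-tagged actors in arrays, replacing contents on entry and clearing through resettable DoOnce gates; middle-volume handlers partly write to CVRightCubes.
; BeginPlay rotates child actors 180° in yaw after a delay.
; Turning is absent: scroll input only prints, and the mapping-context setup is unwired.
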(event OnComponentBeginOverlap(C_V_Left)
  (params (OverlappedComponent :type Primitive%20Component%20Object%20Reference) (OtherActor :type Actor%20Object%20Reference) (OtherComp :type Primitive%20Component%20Object%20Reference) (OtherBodyIndex :type Integer) (bFromSweep :type Boolean) (SweepResult :type Hit%20Result%20Structure%20%28by%20ref%29))
  ;[1 0.9906 0.9844] VerticalArrays
  ;;[0 0.0625 1] VLArrayFill
  (if (Actor|ActorHasTag OtherActor "Cube")
    (for _array_element (Utilities|Array|MakeArray OtherActor)
      (Variables|Arrays/DontTouch|SetC_V_Left_Cubes (Utilities|Array|MakeArray _array_element))
      (Development|PrintString "Ready03"))
    (CallFunction|ResetVL)))

(event OnComponentBeginOverlap(C_H_Mid)
  (params (OverlappedComponent :type Primitive%20Component%20Object%20Reference) (OtherActor :type Actor%20Object%20Reference) (OtherComp :type Primitive%20Component%20Object%20Reference) (OtherBodyIndex :type Integer) (bFromSweep :type Boolean) (SweepResult :type Hit%20Result%20Structure%20%28by%20ref%29))
  ;[0.07812 0 1] Horizontal_Arrays
  ;;[0 1 0.4609] MH_ArrayFill
  (if (Actor|ActorHasTag OtherActor "Cube")
    (for _array_element (Utilities|Array|MakeArray OtherActor)
      (bind _output_get (Variables|Arrays/DontTouch|SetC_V_Right_Cubes (Utilities|Array|MakeArray _array_element)))
      (Development|PrintString "Ready06"))
    (CallFunction|ResetHM)))

(event OnComponentEndOverlap(C_H_Mid)
  (params (OverlappedComponent :type Primitive%20Component%20Object%20Reference) (OtherActor :type Actor%20Object%20Reference) (OtherComp :type Primitive%20Component%20Object%20Reference) (OtherBodyIndex :type Integer))
  ;[0.07812 0 1] Horizontal_Arrays
  ;;[0 1 0.4609] MH_ArrayFill
  (if (Actor|ActorHasTag OtherActor "Cube")
    (Utilities|FlowControl|DoOnce true
      (:Completed
        (Utilities|Array|Clear (stale OnComponentBeginOverlap(C_H_Mid) _output_get))))))

(event OnComponentBeginOverlap(C_H_Bottom)
  (params (OverlappedComponent :type Primitive%20Component%20Object%20Reference) (OtherActor :type Actor%20Object%20Reference) (OtherComp :type Primitive%20Component%20Object%20Reference) (OtherBodyIndex :type Integer) (bFromSweep :type Boolean) (SweepResult :type Hit%20Result%20Structure%20%28by%20ref%29))
  ;[0.07812 0 1] Horizontal_Arrays
  ;;[0 1 1] BH_ArrayFill
  (if (Actor|ActorHasTag OtherActor "Cube")
    (for _array_element (Utilities|Array|MakeArray OtherActor)
      (bind _output_get (Variables|Arrays/DontTouch|SetC_H_Bottom_Cubes (Utilities|Array|MakeArray _array_element)))
      (Development|PrintString "Ready05"))
    (CallFunction|ResetBH)))

(event OnComponentEndOverlap(C_H_Bottom)
  (params (OverlappedComponent :type Primitive%20Component%20Object%20Reference) (OtherActor :type Actor%20Object%20Reference) (OtherComp :type Primitive%20Component%20Object%20Reference) (OtherBodyIndex :type Integer))
  ;[0.07812 0 1] Horizontal_Arrays
  ;;[0 1 1] BH_ArrayFill
  (if (Actor|ActorHasTag OtherActor "Cube")
    (Utilities|FlowControl|DoOnce true
      (:Completed
        (Utilities|Array|Clear (stale OnComponentBeginOverlap(C_H_Bottom) _output_get))))))

(event OnComponentEndOverlap(C_V_Left)
  (params (OverlappedComponent :type Primitive%20Component%20Object%20Reference) (OtherActor :type Actor%20Object%20Reference) (OtherComp :type Primitive%20Component%20Object%20Reference) (OtherBodyIndex :type Integer))
  ;[1 0.9906 0.9844] VerticalArrays
  ;;[0 0.0625 1] VLArrayFill
  (if (Actor|ActorHasTag OtherActor "Cube")
    (Utilities|FlowControl|DoOnce true
      (:Completed
        (Utilities|Array|Clear (Variables|Arrays/DontTouch|GetC_V_Left_Cubes))
        (Development|PrintString "IM CLEAR")))))

(event OnComponentBeginOverlap(C_V_Right)
  (params (OverlappedComponent :type Primitive%20Component%20Object%20Reference) (OtherActor :type Actor%20Object%20Reference) (OtherComp :type Primitive%20Component%20Object%20Reference) (OtherBodyIndex :type Integer) (bFromSweep :type Boolean) (SweepResult :type Hit%20Result%20Structure%20%28by%20ref%29))
  ;[1 0.9906 0.9844] VerticalArrays
  ;;[0 1 0.7656] VRArrayFill
  (if (Actor|ActorHasTag OtherActor "Cube")
    (for _array_element (Utilities|Array|MakeArray OtherActor)
      (Variables|Arrays/DontTouch|SetC_V_Right_Cubes (Utilities|Array|MakeArray _array_element))
      (Development|PrintString "Ready02"))
    (CallFunction|ResetVR)))

(event OnComponentEndOverlap(C_V_Right)
  (params (OverlappedComponent :type Primitive%20Component%20Object%20Reference) (OtherActor :type Actor%20Object%20Reference) (OtherComp :type Primitive%20Component%20Object%20Reference) (OtherBodyIndex :type Integer))
  ;[1 0.9906 0.9844] VerticalArrays
  ;;[0 1 0.7656] VRArrayFill
  (if (Actor|ActorHasTag OtherActor "Cube")
    (Utilities|FlowControl|DoOnce true
      (:Completed
        (Utilities|Array|Clear (Variables|Arrays/DontTouch|GetC_V_Right_Cubes))))))

(event OnComponentBeginOverlap(C_V_Mid)
  (params (OverlappedComponent :type Primitive%20Component%20Object%20Reference) (OtherActor :type Actor%20Object%20Reference) (OtherComp :type Primitive%20Component%20Object%20Reference) (OtherBodyIndex :type Integer) (bFromSweep :type Boolean) (SweepResult :type Hit%20Result%20Structure%20%28by%20ref%29))
  ;[1 0.9906 0.9844] VerticalArrays
  ;;[0.6875 0 1] VMArrayFill
  (if (Actor|ActorHasTag OtherActor "Cube")
    (for _array_element (Utilities|Array|MakeArray OtherActor)
      (Variables|Arrays/DontTouch|SetC_V_Mid_Cubes (Utilities|Array|MakeArray _array_element))
      (Development|PrintString "Ready01"))
    (CallFunction|ResetVM)))

(event OnComponentEndOverlap(C_V_Mid)
  (params (OverlappedComponent :type Primitive%20Component%20Object%20Reference) (OtherActor :type Actor%20Object%20Reference) (OtherComp :type Primitive%20Component%20Object%20Reference) (OtherBodyIndex :type Integer))
  ;[1 0.9906 0.9844] VerticalArrays
  ;;[0.6875 0 1] VMArrayFill
  (if (Actor|ActorHasTag OtherActor "Cube")
    (Utilities|FlowControl|DoOnce true
      (:Completed
        (Utilities|Array|Clear (Variables|Arrays/DontTouch|GetC_V_Right_Cubes))))))

(event OnComponentEndOverlap(C_H_Top)
  (params (OverlappedComponent :type Primitive%20Component%20Object%20Reference) (OtherActor :type Actor%20Object%20Reference) (OtherComp :type Primitive%20Component%20Object%20Reference) (OtherBodyIndex :type Integer))
  ;[0.07812 0 1] Horizontal_Arrays
  ;;[0.4531 1 0] TH_ArrayFill
  (if (Actor|ActorHasTag OtherActor "Cube")
    (Utilities|FlowControl|DoOnce true
      (:Completed
        (Utilities|Array|Clear (stale OnComponentBeginOverlap(C_H_Top) _output_get))))))

(event OnComponentBeginOverlap(C_H_Top)
  (params (OverlappedComponent :type Primitive%20Component%20Object%20Reference) (OtherActor :type Actor%20Object%20Reference) (OtherComp :type Primitive%20Component%20Object%20Reference) (OtherBodyIndex :type Integer) (bFromSweep :type Boolean) (SweepResult :type Hit%20Result%20Structure%20%28by%20ref%29))
  ;[0.07812 0 1] Horizontal_Arrays
  ;;[0.4531 1 0] TH_ArrayFill
  (if (Actor|ActorHasTag OtherActor "Cube")
    (for _array_element (Utilities|Array|MakeArray OtherActor)
      (bind _output_get (Variables|Arrays/DontTouch|SetC_H_Top_Cubes (Utilities|Array|MakeArray _array_element)))
      (Development|PrintString "Ready04"))
    (CallFunction|ResetTH)))

(event Custom|InitSingleCubes
  ;[0.2422 0 1] InitSingleCubes
  (Utilities|FlowControl|Delay 3.0)
  (for _array_element (Actor|GetAllChildActors self true)
    (Transformation|AddRelativeRotation (Variables|/Script/Engine.Actor|GetRootComponent _array_element) "180.000000,0.000000,0.000000" false false)))

(event Custom|ResetTH
  ;[0.07812 0 1] Horizontal_Arrays
  ;;[0.4531 1 0] TH_ArrayFill
  (Utilities|FlowControl|DoOnce true) ; enters at Reset
)

(event Custom|ResetBH
  ;[0.07812 0 1] Horizontal_Arrays
  ;;[0 1 1] BH_ArrayFill
  (Utilities|FlowControl|DoOnce true) ; enters at Reset
)

(event Custom|ResetVL
  ;[1 0.9906 0.9844] VerticalArrays
  ;;[0 0.0625 1] VLArrayFill
  (Utilities|FlowControl|DoOnce true) ; enters at Reset
)

(event Custom|SetupInput
  (params (AsPlayerController :type Player%20Controller%20Object%20Reference))
  ;[0.875 0 1] SetupInput
  (Input|AddMappingContext (PlayerController|LocalPlayerSubsystems|GetEnhancedInputLocalPlayerSubsystem AsPlayerController) "/Game/FPPuzzleGame/Input/IMC_TurnablesMiniGame.IMC_TurnablesMiniGame" 0 "(bIgnoreAllPressedKeysUntilRelease=True,bForceImmediately=False)"))

(event Custom|ResetVR
  ;[1 0.9906 0.9844] VerticalArrays
  ;;[0 1 0.7656] VRArrayFill
  (Utilities|FlowControl|DoOnce true) ; enters at Reset
)

(event Custom|HighlightRow
  (params (0/1/2/3%20 :type Integer))
  (bind _c_h_top (Variables|Default|GetC_H_Top))
  (bind _c_v_left (Variables|Default|GetC_V_Left))
  (if (Variables|Default|GetIsHorizontal)
    (switch int 0/1/2/3%20
      (:0
        ;[0 1 0.1797] HighlightNone
        (Rendering|SetRenderCustomDepth _c_v_left false))
      (:1
        ;[1 0.4688 0] HighlightLeft
        (Rendering|SetRenderCustomDepth _c_v_left true))
      (:2
        ;[1 0.6797 0] HighlightMid
        (Rendering|SetRenderCustomDepth (Variables|Default|GetC_V_Mid) true))
      (:3
        ;[0.5 1 0] HighlightBot
        (Rendering|SetRenderCustomDepth (Variables|Default|GetC_V_Right) true)))
    (else
      (switch int 0/1/2/3%20
        (:0
          ;[0 1 0.1797] HighlightNone
          (Rendering|SetRenderCustomDepth _c_h_top false))
        (:1
          ;[0.2891 1 0] HighlightTop
          (Rendering|SetRenderCustomDepth _c_h_top true))
        (:2
          ;[0.6875 0 1] HighlightMid
          (Rendering|SetRenderCustomDepth (Variables|Default|GetC_H_Mid) true))
        (:3
          ;[1 0.7266 0] HighlightBot
          (Rendering|SetRenderCustomDepth (Variables|Default|GetC_H_Bottom) true))))))

(event Custom|ResetVM
  ;[1 0.9906 0.9844] VerticalArrays
  ;;[0.6875 0 1] VMArrayFill
  (Utilities|FlowControl|DoOnce true) ; enters at Reset
)

(event Custom|ResetHM
  ;[0.07812 0 1] Horizontal_Arrays
  ;;[0 1 0.4609] MH_ArrayFill
  (Utilities|FlowControl|DoOnce true) ; enters at Reset
)

(event Input|EnhancedActionEvents|EnhancedInputActionIA_Scroll
  (params (ActionValue :type Float%20%28double-precision%29) (ElapsedSeconds :type Float%20%28double-precision%29) (TriggeredSeconds :type Float%20%28double-precision%29) (InputAction :type Input%20Action%20Object%20Reference :default "/Game/FPPuzzleGame/Input/IA_Scroll.IA_Scroll"))
  (:Triggered
    (Development|PrintString (Utilities|String|ToString(Float) ActionValue))))

(event EventBeginPlay
  (CallFunction|InitSingleCubes))

(fn ConstructionScript)