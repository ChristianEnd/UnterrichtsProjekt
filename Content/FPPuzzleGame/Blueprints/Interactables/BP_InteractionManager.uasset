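; BP_InteractionManager is a puzzle manager that checks calls from actors against an ordered Actors list and plays a level sequence as the reward.
; Each Call compares the actor to the current position, then advances it, resetting at the list's end.
; IsCombinationRight is inverted, false on a match, and overwritten every call, so only the last comparison decides whether the sequence plays.
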(event EventCall
  (params (Actor :type Actor%20Object%20Reference))
  (bind _sequence (Variables|Default|GetSequence))
  (bind _sequenceplayer (Variables|/Script/LevelSequence.LevelSequenceActor|GetSequencePlayer _sequence))
  (if (> (Utilities|Array|Length (Variables|Default|GetActors)) 0)
    (Utilities|FlowControl|Sequence
      (:then_0
        ;[1 0.6798 0.6198] CheckOrder
        (if (== Actor (Utilities|Array|Get(acopy) (Variables|Default|GetActors) (Variables|Default|GetPosition)))
          (Variables|Default|SetIsCombinationRight false)
          (else
            (Variables|Default|SetIsCombinationRight true))))
      (:then_1
        ;[0.5938 0 1] AddToCheck
        (Math|Integer|IncrementInt (Variables|Default|GetPosition)
          (:%20%20
            ;[0 0.9766 1] ResetList
            (if (>= (Variables|Default|GetPosition) (Utilities|Array|Length (Variables|Default|GetActors)))
              (Variables|Default|SetPosition 0)
              (if (not (Variables|Default|GetIsCombinationRight))
                (Utilities|IsValid _sequenceplayer
                  (:Is%20Valid
                    (Sequencer|Player|Play _sequenceplayer :!class /Script/MovieScene.MovieSceneSequencePlayer)))))))))))

(fn ConstructionScript)