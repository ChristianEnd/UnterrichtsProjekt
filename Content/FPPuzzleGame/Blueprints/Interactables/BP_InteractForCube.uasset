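; BP_InteractForCube is an interactable pawn that opens a terminal minigame, highlighting its upper body via custom depth when focused.
; Interacting makes the player controller possess it and shows the cursor; possession adds the minigame input mapping and pushes the terminal widget to the HUD.
; Cancel re-possesses BP_Player, and unpossession removes the mapping, hides the cursor and cleans the HUD stack.
; Left and right inputs only print debug strings.
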(event Custom|SetupInput
  (params (PlayerController :type Player%20Controller%20Object%20Reference))
  ;[0.8281 0 1] SetupNewInput
  (Input|AddMappingContext (PlayerController|LocalPlayerSubsystems|GetEnhancedInputLocalPlayerSubsystem PlayerController) "/Game/FPPuzzleGame/Input/IMC_Minigame01.IMC_Minigame01" 0 "(bIgnoreAllPressedKeysUntilRelease=True,bForceImmediately=False)"))

(event Input|EnhancedActionEvents|EnhancedInputActionIA_Cancel
  (params (ActionValue :type Boolean) (ElapsedSeconds :type Float%20%28double-precision%29) (TriggeredSeconds :type Float%20%28double-precision%29) (InputAction :type Input%20Action%20Object%20Reference :default "/Game/FPPuzzleGame/Input/IA_Cancel.IA_Cancel"))
  (bind _returnvalue (Game|GetPlayerController 0))
  (:Started
    (bind _returnvalue_2 (Actor|GetActorOfClass "/Game/FPPuzzleGame/Blueprints/Player/BP_Player.BP_Player_C"))
    (Pawn|Possess _returnvalue _returnvalue_2)
    (Class|BPIHUD|CleanGameplayStack(Message) (HUD|GetHUD _returnvalue) "/Game/FPPuzzleGame/UI/Widgets/WBP_Gameplay.WBP_Gameplay_C")))

(event Input|EnhancedActionEvents|EnhancedInputActionIA_Left
  (params (ActionValue :type Boolean) (ElapsedSeconds :type Float%20%28double-precision%29) (TriggeredSeconds :type Float%20%28double-precision%29) (InputAction :type Input%20Action%20Object%20Reference :default "/Game/FPPuzzleGame/Input/IA_Left.IA_Left"))
  (:Started
    (Development|PrintString "links")))

(event Input|EnhancedActionEvents|EnhancedInputActionIA_Right
  (params (ActionValue :type Boolean) (ElapsedSeconds :type Float%20%28double-precision%29) (TriggeredSeconds :type Float%20%28double-precision%29) (InputAction :type Input%20Action%20Object%20Reference :default "/Game/FPPuzzleGame/Input/IA_Right.IA_Right"))
  (:Started
    (Development|PrintString "rechts")))

(event EventSetFocus
  (params (IsFocused :type Boolean))
  (Rendering|SetRenderCustomDepth (Variables|Default|GetUpperBody) IsFocused))

(event EventInteract
  (bind _returnvalue (Game|GetPlayerController 0))
  ;[1 0.4219 0] ChangePossessedPawn
  (Pawn|Possess _returnvalue self)
  (Rendering|SetRenderCustomDepth (Variables|Default|GetUpperBody) false)
  (Variables|/Script/Engine.PlayerController|SetbShowMouseCursor _returnvalue true))

(event EventPossessed
  (params (NewController :type Controller%20Object%20Reference))
  (bind _asplayer_controller (Utilities|Casting|CastToPlayerController NewController))
  (CallFunction|SetupInput _asplayer_controller)
  (Class|BPIHUD|PushtoGameplayStack(Message) (HUD|GetHUD _asplayer_controller) "/Game/FPPuzzleGame/UI/Widgets/WBP_Terminal.WBP_Terminal_C"))

(event EventUnpossessed
  (params (OldController :type Controller%20Object%20Reference))
  (bind _asplayer_controller (Utilities|Casting|CastToPlayerController OldController))
  (Input|RemoveMappingContext (PlayerController|LocalPlayerSubsystems|GetEnhancedInputLocalPlayerSubsystem _asplayer_controller) "/Game/FPPuzzleGame/Input/IMC_Minigame01.IMC_Minigame01" "(bIgnoreAllPressedKeysUntilRelease=True,bForceImmediately=False)")
  (Class|BPIHUD|CleanGameplayStack(Message) (HUD|GetHUD _asplayer_controller) "/Game/FPPuzzleGame/UI/Widgets/WBP_Gameplay.WBP_Gameplay_C")
  (Variables|/Script/Engine.PlayerController|SetbShowMouseCursor _asplayer_controller false))

(fn ConstructionScript)