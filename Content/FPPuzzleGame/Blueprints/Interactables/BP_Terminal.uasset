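; Interactable, possessable terminal for a first-person puzzle game, where the player cycles three buttons and picks a camera-capture view.
; Left/right inputs move a wrapping index, highlighting the active button through custom depth, and Interact applies the matching capture material to Base.
; Focus outlines LowerBody, Interact clears that outline, and unpossessing resets the button highlight.
; Construction creates a Display dynamic material that these graphs never use; the Back/Cancel HUD cleanup is unwired.
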(event Custom|HighlightButtons
  (params (Position :type Integer) (isActive :type Boolean))
  ;[1 0 0.3984] HighlightSelected
  (Rendering|SetRenderCustomDepth (Utilities|Array|Get(acopy) (Variables|Default|GetButtons) Position) isActive))

(event Input|EnhancedActionEvents|EnhancedInputActionIA_Left
  (params (ActionValue :type Boolean) (ElapsedSeconds :type Float%20%28double-precision%29) (TriggeredSeconds :type Float%20%28double-precision%29) (InputAction :type Input%20Action%20Object%20Reference :default "/Game/FPPuzzleGame/Input/IA_Left.IA_Left"))
  ;[0.9688 1 0] SwitchSelection
  (:Started
    (Utilities|FlowControl|Sequence
      (:then_0
        (CallFunction|HighlightButtons (Variables|Default|GetButtonIndexPosition) false))
      (:then_1
        (bind _result (Math|Integer|IncrementInt (Variables|Default|GetButtonIndexPosition))
          (:%20%20
            (if (== _result 3)
              (Variables|Default|SetButtonIndexPosition (- (Utilities|Array|Length (Variables|Default|GetButtons)) _result))))))
      (:then_2
        (CallFunction|HighlightButtons (Variables|Default|GetButtonIndexPosition) true)))))

(event Input|EnhancedActionEvents|EnhancedInputActionIA_Right
  (params (ActionValue :type Boolean) (ElapsedSeconds :type Float%20%28double-precision%29) (TriggeredSeconds :type Float%20%28double-precision%29) (InputAction :type Input%20Action%20Object%20Reference :default "/Game/FPPuzzleGame/Input/IA_Right.IA_Right"))
  ;[0.9688 1 0] SwitchSelection
  (:Started
    (Utilities|FlowControl|Sequence
      (:then_0
        (CallFunction|HighlightButtons (Variables|Default|GetButtonIndexPosition) false))
      (:then_1
        (bind _result (Math|Integer|DecrementInt (Variables|Default|GetButtonIndexPosition))
          (:%20%20
            (Variables|Default|SetButtonIndexPosition _result)
            (if (== _result -1)
              (bind _result_2 (Math|Integer|DecrementInt (Utilities|Array|Length (Variables|Default|GetButtons)))
                (:%20%20
                  (Variables|Default|SetButtonIndexPosition _result_2)))))))
      (:then_2
        (CallFunction|HighlightButtons (Variables|Default|GetButtonIndexPosition) true)))))

(event Input|EnhancedActionEvents|EnhancedInputActionIA_Interact
  (params (ActionValue :type Boolean) (ElapsedSeconds :type Float%20%28double-precision%29) (TriggeredSeconds :type Float%20%28double-precision%29) (InputAction :type Input%20Action%20Object%20Reference :default "/Game/FPPuzzleGame/Input/IA_Interact.IA_Interact"))
  ;[0.9219 1 0] Interact
  (:Started
    (Rendering|Material|SetMaterial (Variables|Default|GetBase) 0 (Utilities|Select :Index (Variables|Default|GetButtonIndexPosition) :Option%200 "/Game/FPPuzzleGame/Materials/M_CameraCapture_Inst.M_CameraCapture_Inst" :Option%201 "/Game/FPPuzzleGame/Materials/M_CameraCapture_Inst1.M_CameraCapture_Inst1" :Option%202 "/Game/FPPuzzleGame/Materials/M_CameraCapture_Inst2.M_CameraCapture_Inst2"))))

(event EventBeginPlay
  ;[0.7344 0 1] FillButtonArray
  (Variables|Default|SetButtons (Utilities|Array|MakeArray (Variables|Default|GetButton01) (Variables|Default|GetButton02) (Variables|Default|GetButton03))))

(event EventUnpossessed
  (params (OldController :type Controller%20Object%20Reference))
  (|CallParentFunction OldController)
  ;[0 1 0.3203] ResetButtonHighlight
  (CallFunction|HighlightButtons (Variables|Default|GetButtonIndexPosition) false))

(event EventSetFocus
  (params (IsFocused :type Boolean))
  ;[0 1 0.6953] SetFocus
  (|CallParentFunction IsFocused)
  (Rendering|SetRenderCustomDepth (Variables|Default|GetLowerBody) IsFocused))

(event EventInteract
  (|CallParentFunction)
  ;[1 0.4219 0] ChangePossessedPawn
  (Rendering|SetRenderCustomDepth (Variables|Default|GetLowerBody) false))

(fn ConstructionScript
  (bind _returnvalue (Rendering|Material|CreateDynamicMaterialInstance (Variables|Default|GetDisplay) 0 0 "None" :!class /Script/Engine.PrimitiveComponent))
  (Variables|Default|SetDynMat _returnvalue))