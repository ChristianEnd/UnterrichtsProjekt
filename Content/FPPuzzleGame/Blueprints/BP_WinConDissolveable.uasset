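; BP_WinConDissolveable is a puzzle cube that dissolves once its win-condition counter reaches WinConAmount.
; Each WinConActivate call increments the counter, and a match plays a timeline that drives the Dissolve parameter on a dynamic material created in the construction script.
; It also carries controls for the ToControl actors: Select steps the index and clears the previous actor's custom depth, while Turn yaws the selected one.
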(event Custom|DissolveMaterial
  ;[1 1 1] DissolveEvent
  (bind _alpha (Timeline|Ani PlayFromStart)
    (:Update
      (Rendering|Material|SetScalarParameterValue (Variables|Default|GetM_Dynamic_Dissolve) "Dissolve" (Math|Float|Lerp 1.0 -1.0 _alpha) :!class /Script/Engine.MaterialInstanceDynamic))))

(event Custom|Turn
  (params (TurnAmount :type Float%20%28double-precision%29))
  (bind _turnmultiplier (Variables|Default|GetTurnMultiplier))
  (bind _tocontrol (Variables|Default|GetToControl))
  (bind _selected (Variables|Default|GetSelected))
  (bind _output (Utilities|Array|Get(acopy) _tocontrol _selected))
  (bind _returnvalue (* TurnAmount _turnmultiplier))
  (bind _rootcomponent (Variables|/Script/Engine.Actor|GetRootComponent _output))
  ;[1 1 1] TurnDirectional
  (if (> TurnAmount 0.0)
    (Transformation|AddRelativeRotation _rootcomponent (Math|Rotator|MakeRotator 0.0 0.0 _returnvalue) false false)
    (else
      (Transformation|AddRelativeRotation _rootcomponent (Math|Rotator|MakeRotator 0.0 0.0 (- _returnvalue 1.0)) false false))))

(event Custom|Select
  (params (Direction :type Float%20%28double-precision%29))
  (Utilities|FlowControl|Sequence
    (:then_0
      (Rendering|SetRenderCustomDepth (Utilities|Array|Get(acopy) (Actor|GetComponentsByClass (Utilities|Array|Get(acopy) (Variables|Default|GetToControl) (Variables|Default|GetSelected)) "/Script/Engine.PrimitiveComponent")) false))
    (:then_1
      (if (> Direction 0.0)
        (Variables|Default|SetSelected (+ (Variables|Default|GetSelected) 1))
        (else
          (Variables|Default|SetSelected (- (Variables|Default|GetSelected) 1)))))))

(event EventWinConActivate
  ;[1 1 1] WinConCounter
  (bind _output_get (Variables|Default|SetCounter (+ (Variables|Default|GetCounter) 1)))
  (if (== _output_get (Variables|Default|GetWinConAmount))
    (CallFunction|DissolveMaterial)))

(event EventBeginPlay
  ;[1 1 1] PlayRate
  (Components|Timeline|SetPlayRate (Variables|Default|GetAni) (Variables|Default|GetPlayRateDissolve))
  ;[1 1 1] TurnablesAmountSet
  (Variables|Default|SetCounter 0)
  (Variables|Default|SetSelected (- (Utilities|Array|Length (Variables|Default|GetToControl)) 1)))

(fn ConstructionScript
  (bind _returnvalue (Rendering|Material|CreateDynamicMaterialInstance "/Game/FPPuzzleGame/Materials/Translucent/M_Dissolve_Red.M_Dissolve_Red" "None" "None" :!class /Script/Engine.KismetMaterialLibrary))
  (bind _output_get (Variables|Default|SetM_Dynamic_Dissolve _returnvalue))
  (Rendering|Material|SetMaterial (Variables|Default|GetCube) 0 _output_get))