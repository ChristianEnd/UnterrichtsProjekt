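; BP_Possessable is an interactable pawn that the player takes control of on Interact, using a minigame input context.
; Interacting clears focus and makes player 0 possess it, which adds IMC_Minigame01 and pushes its widget onto the HUD's gameplay stack.
; Cancel hands possession back to the BP_Player found in the level.
; Unpossessing removes the mapping context and cleans the gameplay stack to WBP_Gameplay.
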(event Custom|SetupInput
  (params (PlayerController :type Player%20Controller%20Object%20Reference))
  ;[0.5 1 0] SetupInput
  (Input|AddMappingContext (PlayerController|LocalPlayerSubsystems|GetEnhancedInputLocalPlayerSubsystem PlayerController) "/Game/FPPuzzleGame/Input/IMC_Minigame01.IMC_Minigame01" 0 "(bIgnoreAllPressedKeysUntilRelease=True,bForceImmediately=False)"))

(event Input|EnhancedActionEvents|EnhancedInputActionIA_Cancel
  (params (ActionValue :type Boolean) (ElapsedSeconds :type Float%20%28double-precision%29) (TriggeredSeconds :type Float%20%28double-precision%29) (InputAction :type Input%20Action%20Object%20Reference :default "/Game/FPPuzzleGame/Input/IA_Cancel.IA_Cancel"))
  (bind _returnvalue (Game|GetPlayerController 0))
  ;[1 0.4453 0] Back/Cancel
  (:Started
    (bind _returnvalue_2 (Actor|GetActorOfClass "/Game/FPPuzzleGame/Blueprints/Player/BP_Player.BP_Player_C"))
    (Pawn|Possess _returnvalue _returnvalue_2)
    (Class|BPIHUD|CleanGameplayStack(Message) (HUD|GetHUD _returnvalue) "/Game/FPPuzzleGame/UI/Widgets/WBP_Gameplay.WBP_Gameplay_C")))

(event EventInteract
  ;[0 0.2266 1] Interact
  (Pawn|Possess (Game|GetPlayerController 0) self)
  (CallFunction|SetFocus false))

(event EventPossessed
  (params (NewController :type Controller%20Object%20Reference))
  ;[0.4297 0 1] Possess
  (bind _asplayer_controller (Utilities|Casting|CastToPlayerController NewController))
  (CallFunction|SetupInput _asplayer_controller)
  (Class|BPIHUD|PushtoGameplayStack(Message) (HUD|GetHUD _asplayer_controller) (Variables|Default|GetWidget)))

(event EventUnpossessed
  (params (OldController :type Controller%20Object%20Reference))
  ;[0 0.5312 1] Unpossess
  (bind _asplayer_controller (Utilities|Casting|CastToPlayerController OldController))
  (Input|RemoveMappingContext (PlayerController|LocalPlayerSubsystems|GetEnhancedInputLocalPlayerSubsystem _asplayer_controller) "/Game/FPPuzzleGame/Input/IMC_Minigame01.IMC_Minigame01" "(bIgnoreAllPressedKeysUntilRelease=True,bForceImmediately=False)")
  (Class|BPIHUD|CleanGameplayStack(Message) (HUD|GetHUD _asplayer_controller) "/Game/FPPuzzleGame/UI/Widgets/WBP_Gameplay.WBP_Gameplay_C"))

(fn ConstructionScript)