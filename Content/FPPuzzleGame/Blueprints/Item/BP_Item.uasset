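; BP_Item is a pickup actor that the player collects into their inventory.
; The construction script looks up the Item's data table row and applies that row's mesh.
; SetFocus toggles custom depth rendering on the mesh to mark focus.
; Interact finds BP_Player by class, adds the Item to its BPInventoryComponent, then destroys the actor.
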(event EventSetFocus
  (params (IsFocused :type Boolean))
  (Rendering|SetRenderCustomDepth (Variables|Default|GetMesh) IsFocused))

(event EventInteract
  (bind _returnvalue (Actor|GetActorOfClass "/Game/FPPuzzleGame/Blueprints/Player/BP_Player.BP_Player_C"))
  (Default|AddItem (Variables|/Game/FPPuzzleGame/Blueprints/Player/BP_Player.BP_Player_C|GetBP_InventoryComponent _returnvalue) (Variables|Default|GetItem))
  (Actor|DestroyActor))

(fn ConstructionScript
  (bind _item (Variables|Default|GetItem))
  (bind (_datatable _rowname) (Utilities|Struct|BreakDataTableRowHandle _item))
  (bind _returnvalue (Utilities|GetDataTableRow _datatable _rowname)
    (:then
      (Components|StaticMesh|SetStaticMesh (Variables|Default|GetMesh) (.Mesh (Utilities|Struct|BreakSTRUCT_Item _returnvalue))))))