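; BP_Keypad is an interactable puzzle keypad with twelve buttons (digits, Delete and Enter) navigated by directional input.
; Focus outlines the keypad and Interact highlights the current button, both through custom depth rendering.
; Left, Right, Up and Down actions step a flat index over a three-column grid, using per-index edge rules and a clamp.
; The button press handler switches on the index but has no actions yet.
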(event Custom|SetupButtons
  ;[1 0.8672 0] SetupButtons
  (Variables|Default|SetButtons (Utilities|Array|MakeArray (Variables|Default|GetB01) (Variables|Default|GetB02) (Variables|Default|GetB03) (Variables|Default|GetB04) (Variables|Default|GetB05) (Variables|Default|GetB06) (Variables|Default|GetB07) (Variables|Default|GetB08) (Variables|Default|GetB09) (Variables|Default|GetDelete) (Variables|Default|GetB00) (Variables|Default|GetEnter))))

(event Custom|HighlightButton
  (params (isActive :type Boolean) (Pos :type Integer))
  ;[0 1 0.6016] HighlightButton
  (Rendering|SetRenderCustomDepth (Utilities|Array|Get(acopy) (Variables|Default|GetButtons) Pos) isActive))

(event Custom|ButtonPressValueEvents
  (switch int (Variables|Default|GetCurrentButtonIndex)))

(event Custom|SecureIndex
  ;[1 0.3516 0] SecureIndex
  (Development|PrintString (Utilities|String|ToString(Integer) (Variables|Default|GetCurrentButtonIndex)))
  (if (>= (Variables|Default|GetCurrentButtonIndex) 11)
    (Variables|Default|SetCurrentButtonIndex 11))
  (if (<= (Variables|Default|GetCurrentButtonIndex) 0)
    (Variables|Default|SetCurrentButtonIndex 0)))

(event Custom|CheckMovement
  ;[0 0.01562 1] MovementRestrictions
  (switch int (Variables|Default|GetCurrentButtonIndex)
    (:0
      (Variables|Default|SetIsMoveHorizontalLeftAllowed false)
      (Variables|Default|SetIsMoveHorizontalRightAllowed true)
      (Variables|Default|SetIsMoveVerticalDownAllowed true)
      (Variables|Default|SetIsMoveVerticalUpAllowed false))
    (:1
      (Variables|Default|SetIsMoveHorizontalLeftAllowed true)
      (Variables|Default|SetIsMoveHorizontalRightAllowed true)
      (Variables|Default|SetIsMoveVerticalDownAllowed true)
      (Variables|Default|SetIsMoveVerticalUpAllowed false))
    (:2
      (Variables|Default|SetIsMoveHorizontalLeftAllowed true)
      (Variables|Default|SetIsMoveHorizontalRightAllowed false)
      (Variables|Default|SetIsMoveVerticalDownAllowed true)
      (Variables|Default|SetIsMoveVerticalUpAllowed false))
    (:3
      (Variables|Default|SetIsMoveHorizontalLeftAllowed false)
      (Variables|Default|SetIsMoveHorizontalRightAllowed true)
      (Variables|Default|SetIsMoveVerticalDownAllowed true)
      (Variables|Default|SetIsMoveVerticalUpAllowed true))
    (:4
      (Variables|Default|SetIsMoveHorizontalLeftAllowed true)
      (Variables|Default|SetIsMoveHorizontalRightAllowed true)
      (Variables|Default|SetIsMoveVerticalDownAllowed true)
      (Variables|Default|SetIsMoveVerticalUpAllowed true))
    (:5
      (Variables|Default|SetIsMoveHorizontalLeftAllowed true)
      (Variables|Default|SetIsMoveHorizontalRightAllowed false)
      (Variables|Default|SetIsMoveVerticalDownAllowed true)
      (Variables|Default|SetIsMoveVerticalUpAllowed true))
    (:6
      (Variables|Default|SetIsMoveHorizontalLeftAllowed false)
      (Variables|Default|SetIsMoveHorizontalRightAllowed true)
      (Variables|Default|SetIsMoveVerticalDownAllowed true)
      (Variables|Default|SetIsMoveVerticalUpAllowed true))
    (:7
      (Variables|Default|SetIsMoveHorizontalLeftAllowed true)
      (Variables|Default|SetIsMoveHorizontalRightAllowed true)
      (Variables|Default|SetIsMoveVerticalDownAllowed true)
      (Variables|Default|SetIsMoveVerticalUpAllowed true))
    (:8
      (Variables|Default|SetIsMoveHorizontalLeftAllowed true)
      (Variables|Default|SetIsMoveHorizontalRightAllowed false)
      (Variables|Default|SetIsMoveVerticalDownAllowed true)
      (Variables|Default|SetIsMoveVerticalUpAllowed true))
    (:9
      (Variables|Default|SetIsMoveHorizontalLeftAllowed false)
      (Variables|Default|SetIsMoveHorizontalRightAllowed true)
      (Variables|Default|SetIsMoveVerticalDownAllowed false)
      (Variables|Default|SetIsMoveVerticalUpAllowed true))
    (:10
      (Variables|Default|SetIsMoveHorizontalLeftAllowed true)
      (Variables|Default|SetIsMoveHorizontalRightAllowed true)
      (Variables|Default|SetIsMoveVerticalDownAllowed false)
      (Variables|Default|SetIsMoveVerticalUpAllowed true))
    (:11
      (Variables|Default|SetIsMoveHorizontalLeftAllowed true)
      (Variables|Default|SetIsMoveHorizontalRightAllowed false)
      (Variables|Default|SetIsMoveVerticalDownAllowed false)
      (Variables|Default|SetIsMoveVerticalUpAllowed true))))

(event Input|EnhancedActionEvents|EnhancedInputActionIA_Left
  (params (ActionValue :type Boolean) (ElapsedSeconds :type Float%20%28double-precision%29) (TriggeredSeconds :type Float%20%28double-precision%29) (InputAction :type Input%20Action%20Object%20Reference :default "/Game/FPPuzzleGame/Input/IA_Left.IA_Left"))
  ;[1 0 0.4453] Left
  (:Started
    (Utilities|FlowControl|Sequence
      (:then_0
        ;;[0.2188 0 1] DeselectAndCheckMovement
        (CallFunction|HighlightButton false (Variables|Default|GetCurrentButtonIndex))
        (CallFunction|CheckMovement))
      (:then_1
        ;;[0 0.4375 1] IsAllowed
        (if (Variables|Default|GetIsMoveHorizontalLeftAllowed)
          ;;[0.9688 1 0] Direction
          (Variables|Default|SetCurrentButtonIndex (- (Variables|Default|GetCurrentButtonIndex) 1))))
      (:then_2
        (CallFunction|SecureIndex))
      (:then_3
        ;;[0 0.2734 1] HighlightNew
        (CallFunction|HighlightButton true (Variables|Default|GetCurrentButtonIndex))))))

(event Input|EnhancedActionEvents|EnhancedInputActionIA_Right
  (params (ActionValue :type Boolean) (ElapsedSeconds :type Float%20%28double-precision%29) (TriggeredSeconds :type Float%20%28double-precision%29) (InputAction :type Input%20Action%20Object%20Reference :default "/Game/FPPuzzleGame/Input/IA_Right.IA_Right"))
  ;[0 0.5078 1] Right
  (:Started
    (Utilities|FlowControl|Sequence
      (:then_0
        ;;[1 0 0.5859] DeselectAndCHeckMove
        (CallFunction|HighlightButton false (Variables|Default|GetCurrentButtonIndex))
        (CallFunction|CheckMovement))
      (:then_1
        ;;[0.2891 1 0] IsAllowed
        (if (Variables|Default|GetIsMoveHorizontalRightAllowed)
          ;;[0.4297 0 1] Direction
          (Variables|Default|SetCurrentButtonIndex (+ (Variables|Default|GetCurrentButtonIndex) 1))))
      (:then_2
        (CallFunction|SecureIndex))
      (:then_3
        ;;[0 1 0.8359] HighlightNew
        (CallFunction|HighlightButton true (Variables|Default|GetCurrentButtonIndex))))))

(event Input|EnhancedActionEvents|EnhancedInputActionIA_Up
  (params (ActionValue :type Boolean) (ElapsedSeconds :type Float%20%28double-precision%29) (TriggeredSeconds :type Float%20%28double-precision%29) (InputAction :type Input%20Action%20Object%20Reference :default "/Game/FPPuzzleGame/Input/IA_Up.IA_Up"))
  ;[1 0.2344 0] up
  (:Started
    (Utilities|FlowControl|Sequence
      (:then_0
        (CallFunction|HighlightButton false (Variables|Default|GetCurrentButtonIndex))
        (CallFunction|CheckMovement))
      (:then_1
        ;;[0 1 0.9062] IsAllowed
        (if (Variables|Default|GetIsMoveVerticalUpAllowed)
          ;;[0 1 0.01562] Direction
          (Variables|Default|SetCurrentButtonIndex (- (Variables|Default|GetCurrentButtonIndex) 3))))
      (:then_2
        (CallFunction|SecureIndex))
      (:then_3
        (CallFunction|HighlightButton true (Variables|Default|GetCurrentButtonIndex))))))

(event Input|EnhancedActionEvents|EnhancedInputActionIA_Down
  (params (ActionValue :type Boolean) (ElapsedSeconds :type Float%20%28double-precision%29) (TriggeredSeconds :type Float%20%28double-precision%29) (InputAction :type Input%20Action%20Object%20Reference :default "/Game/FPPuzzleGame/Input/IA_Down.IA_Down"))
  ;[0 1 0.7422] Down
  (:Started
    (Utilities|FlowControl|Sequence
      (:then_0
        ;;[0 0.4141 1] DeselectAndCheckMove
        (CallFunction|HighlightButton false (Variables|Default|GetCurrentButtonIndex))
        (CallFunction|CheckMovement))
      (:then_1
        ;;[0 1 0.3203] IsAllowed
        (if (Variables|Default|GetIsMoveVerticalDownAllowed)
          ;;[0 0.9766 1] Direction
          (Variables|Default|SetCurrentButtonIndex (+ (Variables|Default|GetCurrentButtonIndex) 3))))
      (:then_2
        (CallFunction|SecureIndex))
      (:then_3
        (CallFunction|HighlightButton true (Variables|Default|GetCurrentButtonIndex))))))

(event EventSetFocus
  (params (IsFocused :type Boolean))
  ;[0.9688 1 0] ParentInit
  (|CallParentFunction IsFocused)
  (Rendering|SetRenderCustomDepth (Variables|Default|GetKeypad_Cube) IsFocused))

(event EventInteract
  ;[0.9688 1 0] ParentInit
  (|CallParentFunction)
  (CallFunction|HighlightButton true (Variables|Default|GetCurrentButtonIndex)))

(event EventBeginPlay
  ;[0.9688 1 0] ParentInit
  (CallFunction|SetupButtons))

(fn ConstructionScript)