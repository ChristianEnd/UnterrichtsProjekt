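; Simon Says puzzle actor: the player watches a random colour light sequence, then repeats it.
; Overlap triggers select the start control or colour button for Interact, and SetFocus outlines it via custom depth.
; Start replays the playlist through delayed self-calls and material swaps, then CheckNode compares each press.
; A mistake flashes all lights red and resets difficulty, while a completed round raises it until WinCondition prints a win.
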(event OnComponentBeginOverlap(Trigger)
  (params (OverlappedComponent :type Primitive%20Component%20Object%20Reference) (OtherActor :type Actor%20Object%20Reference) (OtherComp :type Primitive%20Component%20Object%20Reference) (OtherBodyIndex :type Integer) (bFromSweep :type Boolean) (SweepResult :type Hit%20Result%20Structure%20%28by%20ref%29))
  ;[0.6875 0 1] Collision
  (Variables|State|SetinRange (Utilities|DoesObjectImplementInterface OtherActor "/Game/FPPuzzleGame/Blueprints/Interfaces/BPI_Player.BPI_Player_C"))
  (Variables|ColorCode|SetSwitchIntColor 0))

(event OnComponentEndOverlap(Trigger)
  (params (OverlappedComponent :type Primitive%20Component%20Object%20Reference) (OtherActor :type Actor%20Object%20Reference) (OtherComp :type Primitive%20Component%20Object%20Reference) (OtherBodyIndex :type Integer))
  ;[0.6875 0 1] Collision
  (if (Utilities|DoesObjectImplementInterface OtherActor "/Game/FPPuzzleGame/Blueprints/Interfaces/BPI_Player.BPI_Player_C")
    (Variables|State|SetinRange false)))

(event OnComponentEndOverlap(BlueTrigger)
  (params (OverlappedComponent :type Primitive%20Component%20Object%20Reference) (OtherActor :type Actor%20Object%20Reference) (OtherComp :type Primitive%20Component%20Object%20Reference) (OtherBodyIndex :type Integer))
  ;[0.8047 1 0] SettingSelectedColor
  (if (Utilities|DoesObjectImplementInterface OtherActor "/Game/FPPuzzleGame/Blueprints/Interfaces/BPI_Player.BPI_Player_C")
    (Variables|State|SetinRange false)
    (Rendering|SetRenderCustomDepth (Variables|Default|GetBlueHolder) false)))

(event OnComponentEndOverlap(YellowTrigger)
  (params (OverlappedComponent :type Primitive%20Component%20Object%20Reference) (OtherActor :type Actor%20Object%20Reference) (OtherComp :type Primitive%20Component%20Object%20Reference) (OtherBodyIndex :type Integer))
  ;[0.8047 1 0] SettingSelectedColor
  (if (Utilities|DoesObjectImplementInterface OtherActor "/Game/FPPuzzleGame/Blueprints/Interfaces/BPI_Player.BPI_Player_C")
    (Variables|State|SetinRange false)
    (Rendering|SetRenderCustomDepth (Variables|Default|GetYellowHolder) false)))

(event OnComponentEndOverlap(RedTrigger)
  (params (OverlappedComponent :type Primitive%20Component%20Object%20Reference) (OtherActor :type Actor%20Object%20Reference) (OtherComp :type Primitive%20Component%20Object%20Reference) (OtherBodyIndex :type Integer))
  ;[0.8047 1 0] SettingSelectedColor
  (if (Utilities|DoesObjectImplementInterface OtherActor "/Game/FPPuzzleGame/Blueprints/Interfaces/BPI_Player.BPI_Player_C")
    (Variables|State|SetinRange false)
    (Rendering|SetRenderCustomDepth (Variables|Default|GetRedHolder) false)))

(event OnComponentEndOverlap(GreenTrigger)
  (params (OverlappedComponent :type Primitive%20Component%20Object%20Reference) (OtherActor :type Actor%20Object%20Reference) (OtherComp :type Primitive%20Component%20Object%20Reference) (OtherBodyIndex :type Integer))
  ;[0.8047 1 0] SettingSelectedColor
  (if (Utilities|DoesObjectImplementInterface OtherActor "/Game/FPPuzzleGame/Blueprints/Interfaces/BPI_Player.BPI_Player_C")
    (Variables|State|SetinRange false)
    (Rendering|SetRenderCustomDepth (Variables|Default|GetGreenHolder) false)))

(event OnComponentBeginOverlap(GreenTrigger)
  (params (OverlappedComponent :type Primitive%20Component%20Object%20Reference) (OtherActor :type Actor%20Object%20Reference) (OtherComp :type Primitive%20Component%20Object%20Reference) (OtherBodyIndex :type Integer) (bFromSweep :type Boolean) (SweepResult :type Hit%20Result%20Structure%20%28by%20ref%29))
  ;[0.8047 1 0] SettingSelectedColor
  (Variables|State|SetinRange (Utilities|DoesObjectImplementInterface OtherActor "/Game/FPPuzzleGame/Blueprints/Interfaces/BPI_Player.BPI_Player_C"))
  (Variables|ColorCode|SetSwitchIntColor 3))

(event OnComponentBeginOverlap(BlueTrigger)
  (params (OverlappedComponent :type Primitive%20Component%20Object%20Reference) (OtherActor :type Actor%20Object%20Reference) (OtherComp :type Primitive%20Component%20Object%20Reference) (OtherBodyIndex :type Integer) (bFromSweep :type Boolean) (SweepResult :type Hit%20Result%20Structure%20%28by%20ref%29))
  ;[0.8047 1 0] SettingSelectedColor
  (Variables|State|SetinRange (Utilities|DoesObjectImplementInterface OtherActor "/Game/FPPuzzleGame/Blueprints/Interfaces/BPI_Player.BPI_Player_C"))
  (Variables|ColorCode|SetSwitchIntColor 1))

(event OnComponentBeginOverlap(YellowTrigger)
  (params (OverlappedComponent :type Primitive%20Component%20Object%20Reference) (OtherActor :type Actor%20Object%20Reference) (OtherComp :type Primitive%20Component%20Object%20Reference) (OtherBodyIndex :type Integer) (bFromSweep :type Boolean) (SweepResult :type Hit%20Result%20Structure%20%28by%20ref%29))
  ;[0.8047 1 0] SettingSelectedColor
  (Variables|State|SetinRange (Utilities|DoesObjectImplementInterface OtherActor "/Game/FPPuzzleGame/Blueprints/Interfaces/BPI_Player.BPI_Player_C"))
  (Variables|ColorCode|SetSwitchIntColor 4))

(event OnComponentBeginOverlap(RedTrigger)
  (params (OverlappedComponent :type Primitive%20Component%20Object%20Reference) (OtherActor :type Actor%20Object%20Reference) (OtherComp :type Primitive%20Component%20Object%20Reference) (OtherBodyIndex :type Integer) (bFromSweep :type Boolean) (SweepResult :type Hit%20Result%20Structure%20%28by%20ref%29))
  ;[0.8047 1 0] SettingSelectedColor
  (Variables|State|SetinRange (Utilities|DoesObjectImplementInterface OtherActor "/Game/FPPuzzleGame/Blueprints/Interfaces/BPI_Player.BPI_Player_C"))
  (Variables|ColorCode|SetSwitchIntColor 2))

(event Custom|SetupDifficulty
  ;[0 1 0.7656] SetupDifficulty
  (Utilities|Array|Clear (Variables|Default|GetPlaylist))
  (switch int (Variables|DifficultySettings|GetDifficulty)
    (:1
      (Variables|DifficultySettings|SetToRemember 3)
      (Variables|DifficultySettings|SetSpeed 1.5))
    (:2
      (Variables|DifficultySettings|SetToRemember 5)
      (Variables|DifficultySettings|SetSpeed 1.0))
    (:3
      (Variables|DifficultySettings|SetToRemember 3)
      (Variables|DifficultySettings|SetSpeed 0.5))))

(event Custom|CreatePlaylist
  ;[0.8047 1 0] CreatePlaylist
  (while (< (Utilities|Array|Length (Variables|Default|GetPlaylist)) (Variables|DifficultySettings|GetToRemember))
    (Utilities|Array|Add (Variables|Default|GetPlaylist) (Math|Random|RandomIntegerinRange 0 3))))

(event Custom|Start
  (if (not (Variables|State|GetisListening))
    (Variables|State|SetisPlaying true)
    (if (< (Variables|Default|GetNotesPlayed) (Variables|DifficultySettings|GetToRemember))
      (switch int (Utilities|Array|Get(acopy) (Variables|Default|GetPlaylist) (Variables|Default|GetNotesPlayed))
        (:0
          ;[0 0.5312 1] Blue
          (CallFunction|PlayNotes false (Variables|Default|GetBlueLight) "/Game/FPPuzzleGame/Materials/General/M_MI_E_Blue.M_MI_E_Blue" "/Game/FPPuzzleGame/Materials/General/M_MI_Blue.M_MI_Blue"))
        (:1
          ;[1 0.1068 0.1008] Red
          (CallFunction|PlayNotes false (Variables|Default|GetRedLight) "/Game/FPPuzzleGame/Materials/General/M_MI_E_Red.M_MI_E_Red" "/Game/FPPuzzleGame/Materials/General/M_MI_Red.M_MI_Red"))
        (:2
          ;[0.4399 1 0.1922] Green
          (CallFunction|PlayNotes false (Variables|Default|GetGreenLight) "/Game/FPPuzzleGame/Materials/General/M_MI_E_Green.M_MI_E_Green" "/Game/FPPuzzleGame/Materials/General/M_MI_Green.M_MI_Green"))
        (:3
          ;[1 0.9191 0.05105] Yellow
          (CallFunction|PlayNotes false (Variables|Default|GetYellowLight) "/Game/FPPuzzleGame/Materials/General/M_MI_E_Yellow.M_MI_E_Yellow" "/Game/FPPuzzleGame/Materials/General/M_MI_Yellow.M_MI_Yellow")))
      (Variables|Default|SetNotesPlayed (+ (Variables|Default|GetNotesPlayed) 1))
      (if (< (Variables|Default|GetNotesPlayed) (Variables|DifficultySettings|GetToRemember))
        (Utilities|FlowControl|Delay (Variables|DifficultySettings|GetSpeed))
        (CallFunction|Start)
        (else
          (Variables|State|SetisPlaying false)
          (Variables|State|SetisListening true))))))

(event Custom|PlayNotes
  (params (isFail :type Boolean) (LightObject :type Primitive%20Component%20Object%20Reference) (OnMaterial :type Material%20Interface%20Object%20Reference) (OffMaterial :type Material%20Interface%20Object%20Reference))
  ;[1 0 0.6328] PlayNoteAnim
  (if isFail
    (Rendering|Material|SetMaterial (Variables|Default|GetBlueLight) 0 "/Game/FPPuzzleGame/Materials/General/M_MI_E_Red.M_MI_E_Red")
    (Utilities|FlowControl|Delay 0.5)
    (Rendering|Material|SetMaterial (Variables|Default|GetBlueLight) 0 "/Game/FPPuzzleGame/Materials/General/M_MI_Blue.M_MI_Blue")
    (Rendering|Material|SetMaterial (Variables|Default|GetRedLight) 0 "/Game/FPPuzzleGame/Materials/General/M_MI_Red.M_MI_Red")
    (Rendering|Material|SetMaterial (Variables|Default|GetGreenLight) 0 "/Game/FPPuzzleGame/Materials/General/M_MI_Green.M_MI_Green")
    (Rendering|Material|SetMaterial (Variables|Default|GetYellowLight) 0 "/Game/FPPuzzleGame/Materials/General/M_MI_Yellow.M_MI_Yellow")
    (CallFunction|ResetMiniGame true)
    (else
      (Rendering|Material|SetMaterial LightObject 0 OnMaterial)
      (Utilities|FlowControl|Delay 0.5)
      (Rendering|Material|SetMaterial LightObject 0 OffMaterial))))

(event Custom|CheckWin
  ;[1 0 0.4219] CheckWin
  (if (== (Utilities|Array|Length (Variables|Default|GetPlaylist)) (Utilities|Array|Length (Variables|Default|GetPlayerPlayList)))
    (if (< (Variables|DifficultySettings|GetDifficulty) (Variables|Default|GetWinCondition))
      (Math|Integer|IncrementInt (Variables|DifficultySettings|GetDifficulty)
        (:%20%20
          (CallFunction|ResetMiniGame false)))
      (else
        (Development|PrintString "Win")))))

(event EventInteract
  (bind _switchintcolor (Variables|ColorCode|GetSwitchIntColor))
  (bind _switchintcolor_2 (Variables|ColorCode|GetSwitchIntColor))
  ;[1 0.7756 0.9124] Interaction
  (if (Variables|State|GetinRange)
    (Development|PrintString (Utilities|String|ToString(Integer) _switchintcolor_2))
    (switch int _switchintcolor_2
      (:0
        (if (and (Variables|State|GetisListening) (Variables|State|GetisPlaying))
          (Development|PrintString "StillListeningandPlaying")
          (else
            (CallFunction|SetupDifficulty)
            (CallFunction|CreatePlaylist)
            (CallFunction|Start))))
      (:1
        (bind _isfail (CallFunction|CheckNode _switchintcolor))
        ;;[0 0.5312 1] Blue
        (CallFunction|PlayNotes _isfail (Variables|Default|GetBlueLight) "/Game/FPPuzzleGame/Materials/General/M_MI_E_Blue.M_MI_E_Blue" "/Game/FPPuzzleGame/Materials/General/M_MI_Blue.M_MI_Blue")
        (CallFunction|CheckWin))
      (:2
        (bind _isfail_2 (CallFunction|CheckNode _switchintcolor))
        ;;[1 0.1068 0.1008] Red
        (CallFunction|PlayNotes _isfail_2 (Variables|Default|GetRedLight) "/Game/FPPuzzleGame/Materials/General/M_MI_E_Red.M_MI_E_Red" "/Game/FPPuzzleGame/Materials/General/M_MI_Red.M_MI_Red")
        (CallFunction|CheckWin))
      (:3
        (bind _isfail_3 (CallFunction|CheckNode _switchintcolor))
        ;;[0.4399 1 0.1922] Green
        (CallFunction|PlayNotes _isfail_3 (Variables|Default|GetGreenLight) "/Game/FPPuzzleGame/Materials/General/M_MI_E_Green.M_MI_E_Green" "/Game/FPPuzzleGame/Materials/General/M_MI_Green.M_MI_Green")
        (CallFunction|CheckWin))
      (:4
        (bind _isfail_4 (CallFunction|CheckNode _switchintcolor))
        ;;[1 0.9191 0.05105] Yellow
        (CallFunction|PlayNotes _isfail_4 (Variables|Default|GetYellowLight) "/Game/FPPuzzleGame/Materials/General/M_MI_E_Yellow.M_MI_E_Yellow" "/Game/FPPuzzleGame/Materials/General/M_MI_Yellow.M_MI_Yellow")
        (CallFunction|CheckWin)))))

(event EventSetFocus
  (params (IsFocused :type Boolean))
  ;[1 0.7756 0.9124] Interaction
  (if (Variables|State|GetinRange)
    (switch int (Variables|ColorCode|GetSwitchIntColor)
      (:0
        (Rendering|SetRenderCustomDepth (Variables|Default|GetPlayerTrigger) IsFocused))
      (:1
        (Rendering|SetRenderCustomDepth (Variables|Default|GetBlueHolder) IsFocused))
      (:2
        (Rendering|SetRenderCustomDepth (Variables|Default|GetRedHolder) IsFocused))
      (:3
        (Rendering|SetRenderCustomDepth (Variables|Default|GetGreenHolder) IsFocused))
      (:4
        (Rendering|SetRenderCustomDepth (Variables|Default|GetYellowHolder) IsFocused)))))

(fn ConstructionScript)

(fn CheckNode
  (params (NoteToCheck :type Integer))
  (Utilities|Array|Add (Variables|Default|GetPlayerPlayList) NoteToCheck)
  (return (not (== NoteToCheck (Utilities|Array|Get(acopy) (Variables|Default|GetPlaylist) (- (Utilities|Array|Length (Variables|Default|GetPlayerPlayList)) 1))))))

(fn ResetMiniGame
  (params (isFail :type Boolean))
  (if isFail
    (Variables|State|SetisListening false)
    (Variables|State|SetisPlaying false)
    (Utilities|Array|Clear (Variables|Default|GetPlaylist))
    (Variables|Default|SetNotesPlayed 0)
    (Variables|DifficultySettings|SetToRemember 0)
    (Variables|DifficultySettings|SetDifficulty 1)
    (Utilities|Array|Clear (Variables|Default|GetPlayerPlayList))
    (else
      (Variables|State|SetisListening false)
      (Variables|State|SetisPlaying false)
      (Utilities|Array|Clear (Variables|Default|GetPlaylist))
      (Variables|Default|SetNotesPlayed 0)
      (Variables|DifficultySettings|SetToRemember 0)
      (Utilities|Array|Clear (Variables|Default|GetPlayerPlayList)))))